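; BP_FollowCamera is a camera actor that becomes the first player's view target on BeginPlay and follows a target actor.
; Each tick, if the target is valid, it interpolates toward the target's location plus a scaled offset and sets the camera to a configured world rotation.
; The construction script starts a looping EditorTick timer, but that function is empty.
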(event `self.ReceiveBeginPlay`
  (set `self.bFindCameraComponentWhenViewTarget` true)
  (`PlayerController.SetViewTargetWithBlend` (`GameplayStatics.GetPlayerController` 0) self 0.0 "VTBlend_Linear" 0.0 false))

(event `self.ReceiveTick`
  (params (DeltaSeconds :type "Float (single-precision)"))
  (`/Engine/EditorBlueprintResources/StandardMacros.IsValid` (`self.Target`)
    (:`Is Valid`
      (`self.K2_SetActorLocation` (`KismetMathLibrary.VInterpTo` (`self.K2_GetActorLocation`) (+ (`self.K2_GetActorLocation` (`self.Target`)) (* (`self.Offset`) (`self.Length`))) (`GameplayStatics.GetWorldDeltaSeconds`) (`self.InterpSpeed`)))
      (`SceneComponent.K2_SetWorldRotation` (`self.Camera`) (`self.Angle`) false false))))

(fn `EditorTick`)

(fn `UserConstructionScript`
  (`KismetSystemLibrary.K2_SetTimer` null "EditorTick" 0.01 true))
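; Player character with melee attack, block and item pickup, moving relative to BP_FollowCamera and turning toward mouse or gamepad aim.
; Timelines animate both hands; weapon overlaps during attacks damage BPA_Damageable actors, and blocking halves walk speed.
; Tick selects an in-range BPA_Pickup within the facing cone for BPPickupAgent to grab.
; Holding ThrowRight charges a meter shown only in debug output, with no throw implemented.
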(event `InputAction|ThrowRight`
  (params (Key :type "Key Structure"))
  (:`Pressed`
    (set `self.ThrowRightPressed` true))
  (:`Released`
    (set `self.ThrowRightPressed` false)))

(event `InputAction|Pickup`
  (params (Key :type "Key Structure"))
  (:`Pressed`
    (set `self.PickupPressed` true)
    (bind _selectedpickup (`self.SelectedPickup`)
      (:`then`
        (`/Game/_Game/Blueprints/BPA_Pickup.OnPickup` _selectedpickup self)
        (`/Game/_Game/Blueprints/BPA_PickupAgent.PickupRight` (`self.BP_PickupAgent`) _selectedpickup))
      (:`else`)))
  (:`Released`
    (set `self.PickupPressed` false)))

(event `self.ReceiveBeginPlay`
  (bind _returnvalue (`GameplayStatics.GetActorOfClass` "/Game/_Game/Blueprints/BP_FollowCamera.BP_FollowCamera_C"))
  (set `self.FollowCam` _returnvalue)
  (set `self.Default_R` (`SceneComponent.GetRelativeTransform` (`self.Hand_R`)))
  (set `self.Default_L` (`SceneComponent.GetRelativeTransform` (`self.Hand_L`)))
  (set `self.CanAttack` true)
  (set `CharacterMovementComponent.MaxWalkSpeed` (`self.MoveSpeed`) (`self.CharacterMovement`))
  (set `self.RotationDirection` (`KismetMathLibrary.Normal` (`self.GetActorForwardVector`))))

(event `InputAxis|Move Right / Left`
  (params (AxisValue :type "Float (single-precision)"))
  (bind _returnvalue (`self.GetActorRightVector` (`self.FollowCam`)))
  (`self.AddMovementInput` _returnvalue AxisValue)
  (set `self.MoveRightVec` (* _returnvalue AxisValue)))

(event `InputAxis|Move Forward / Backward`
  (params (AxisValue :type "Float (single-precision)"))
  (bind _returnvalue (`self.GetActorForwardVector` (`self.FollowCam`)))
  (`self.AddMovementInput` _returnvalue AxisValue)
  (set `self.MoveLeftVec` (* _returnvalue AxisValue)))

(event `InputAxis|Turn Right / Left Mouse`
  (params (AxisValue :type "Float (single-precision)"))
  (set `self.RotationDirection` (`KismetMathLibrary.RotateAngleAxis` (`self.RotationDirection`) (* AxisValue (`self.RotationSpeed`)) (0.0 0.0 1.0))))

(event `InputAxis|Turn Right / Left Gamepad`
  (params (AxisValue :type "Float (single-precision)"))
  ;[1 1 1] Forward
  (set `self.RightDir` (* AxisValue (`self.GetActorRightVector` (`self.FollowCam`)))))

(event `InputAxis|Look Up / Down Gamepad`
  (params (AxisValue :type "Float (single-precision)"))
  ;[1 1 1] Right
  (set `self.LeftDir` (* AxisValue (`self.GetActorForwardVector` (`self.FollowCam`)) -1.0)))

(event `InputAction|Attack`
  (params (Key :type "Key Structure"))
  (:`Pressed`
    (if (not (`self.IsBlocking`))
      (if (`self.CanAttack`)
        (set `self.IsAttacking` true)
        (set `self.CanAttack` false)
        (bind (_direction _translation _rotation) (`Timeline|AttackR_Timeline` :`NewTime` 0.0 :!via `PlayFromStart`)
          (:`Update`
            (bind (_x _y _z) (`KismetMathLibrary.BreakVector3f` _rotation))
            (`SceneComponent.K2_SetRelativeLocationAndRotation` (`self.Hand_R`) (+ _translation (.location (`self.Default_R`))) (`KismetMathLibrary.ComposeRotators` (`KismetMathLibrary.MakeRotator` _x _y _z) (.rotation (`self.Default_R`))) false false))
          (:`Finished`
            (set `self.CanAttack` true)
            (set `self.IsAttacking` false)))))))

(event `InputAction|Block`
  (params (Key :type "Key Structure"))
  (:`Pressed`
    (set `self.IsBlocking` true)
    (bind (_direction _translation _rotation) (`Timeline|Block` :!label _label)
      (:`Update`
        (bind (_x _y _z) (`KismetMathLibrary.BreakVector3f` _rotation))
        (`SceneComponent.K2_SetRelativeLocationAndRotation` (`self.Hand_L`) (+ _translation (.location (`self.Default_L`))) (`KismetMathLibrary.ComposeRotators` (`KismetMathLibrary.MakeRotator` _x _y _z) (.rotation (`self.Default_L`))) false false))))
  (:`Released`
    (set `self.IsBlocking` false)
    (goto _label :!via `Reverse`)))

(event `self.ReceiveTick`
  (params (DeltaSeconds :type "Float (single-precision)"))
  (bind _returnvalue (`self.K2_GetActorLocation`))
  (bind _returnvalue_2 (`self.K2_GetActorLocation`))
  (bind _returnvalue_3 (`self.K2_GetActorLocation`))
  (bind (_returnvalue_roll _returnvalue_pitch _returnvalue_yaw) (`KismetMathLibrary.BreakRotator` (`KismetMathLibrary.RInterpTo` (`self.CurrentRotation`) (`KismetMathLibrary.FindLookAtRotation` (`KismetMathLibrary.Vector_Zero`) (`self.RotationDirection`)) (`GameplayStatics.GetWorldDeltaSeconds`) 5.0)))
  (bind (_returnvalue_x _returnvalue_y) (`KismetMathLibrary.BreakVector` (+ _returnvalue_2 (* (`KismetMathLibrary.Normal` (`self.RotationDirection`)) 100.0))))
  (`|ExecutionSequence`
    (:`then_0`
      (`KismetSystemLibrary.DrawDebugLine` _returnvalue_2 (`KismetMathLibrary.MakeVector` _returnvalue_x _returnvalue_y (`.Z` (`KismetMathLibrary.BreakVector3f` _returnvalue_2))) (struct :`R` 1.0 :`A` 1.0) 0.0 4.0)
      (`/Game/_Game/Blueprints/BP_UtilityLib.LogBool` "IsBlocking" (`self.IsBlocking`))
      (`/Game/_Game/Blueprints/BP_UtilityLib.LogBool` "CanAttack" (`self.CanAttack`))
      (`/Game/_Game/Blueprints/BP_UtilityLib.LogVec` "MovementInput" (`self.MovementInput`))
      (`/Game/_Game/Blueprints/BP_UtilityLib.LogVec` "RotationDirection" (`self.RotationDirection`))
      (`KismetSystemLibrary.DrawDebugLine` _returnvalue_3 (+ _returnvalue_3 (* (`KismetMathLibrary.Normal` (`self.MovementInput`)) 75.0)) (struct :`B` 1.0 :`A` 1.0) 0.0 4.0)
      (`KismetSystemLibrary.DrawDebugLine` (+ _returnvalue (0.0 0.0 2.0)) (+ (+ _returnvalue (* (`self.RotationDirection`) (`self.ThrowMeterR`) 100.0)) (0.0 0.0 2.0)) (struct :`G` 0.868849 :`B` 1.0 :`A` 1.0) 0.0 6.0))
    (:`then_1`
      (if (`self.IsBlocking`)
        (set `CharacterMovementComponent.MaxWalkSpeed` (* (`self.MoveSpeed`) 0.5) (`self.CharacterMovement`))
        (else
          (set `CharacterMovementComponent.MaxWalkSpeed` (`self.MoveSpeed`) (`self.CharacterMovement`)))))
    (:`then_2`
      ;[1 1 1] Character Rotation
      (set `self.MovementInput` (+ (`self.MoveRightVec`) (`self.MoveLeftVec`)))
      (bind _output_get (set `self.RotationInput` (+ (`self.LeftDir`) (`self.RightDir`))))
      (if (> (`KismetMathLibrary.VSize` _output_get) 0.0)
        (set `self.RotationDirection` (`self.RotationInput`)))
      (bind _output_get_2 (set `self.CurrentRotation` (`KismetMathLibrary.MakeRotator` 0.0 0.0 _returnvalue_yaw)))
      (`self.K2_SetActorRotation` (`KismetMathLibrary.MakeRotator` 0.0 0.0 (.yaw _output_get_2))))
    (:`then_3`
      (`self.ClosestPickup`)
      (if (`self.ThrowRightPressed`)
        (bind _output_get_3 (set `self.ThrowMeterR` (`KismetMathLibrary.FClamp` (+ (`self.ThrowMeterR`) (`GameplayStatics.GetWorldDeltaSeconds`)))))
        (`/Game/_Game/Blueprints/BP_UtilityLib.LogFloat` "ThrowR" _output_get_3)
        (else
          (bind _output_get_4 (set `self.ThrowMeterR` 0.0))
          (`/Game/_Game/Blueprints/BP_UtilityLib.LogFloat` "ThrowR" _output_get_4))))))

(event `self.Weapon_Collider.OnComponentBeginOverlap`
  (params (OverlappedComponent :type "PrimitiveComponent Object Reference") (OtherActor :type "Actor Object Reference") (OtherComp :type "PrimitiveComponent Object Reference") (OtherBodyIndex :type Integer) (bFromSweep :type Boolean) (SweepResult :type "HitResult Structure (by ref)"))
  (bind _returnvalue (`self.GetComponentByClass` OtherActor "/Game/_Game/Blueprints/BPA_Damageable.BPA_Damageable_C"))
  (if (`self.IsAttacking`)
    (`/Engine/EditorBlueprintResources/StandardMacros.IsValid` _returnvalue
      (:`Is Valid`
        (`/Game/_Game/Blueprints/BPA_Damageable.TakeDamage` _returnvalue 10)))))

(event `self.PickupRange.OnComponentBeginOverlap`
  (params (OverlappedComponent :type "PrimitiveComponent Object Reference") (OtherActor :type "Actor Object Reference") (OtherComp :type "PrimitiveComponent Object Reference") (OtherBodyIndex :type Integer) (bFromSweep :type Boolean) (SweepResult :type "HitResult Structure (by ref)"))
  (bind _returnvalue (`self.GetComponentByClass` OtherActor "/Game/_Game/Blueprints/BPA_Pickup.BPA_Pickup_C"))
  (`/Engine/EditorBlueprintResources/StandardMacros.IsValid` _returnvalue
    (:`Is Valid`
      (`KismetArrayLibrary.Array_AddUnique` (`self.PickupsInRange`) _returnvalue))))

(event `self.PickupRange.OnComponentEndOverlap`
  (params (OverlappedComponent :type "PrimitiveComponent Object Reference") (OtherActor :type "Actor Object Reference") (OtherComp :type "PrimitiveComponent Object Reference") (OtherBodyIndex :type Integer))
  (bind _returnvalue (`self.GetComponentByClass` OtherActor "/Game/_Game/Blueprints/BPA_Pickup.BPA_Pickup_C"))
  (`/Engine/EditorBlueprintResources/StandardMacros.IsValid` _returnvalue
    (:`Is Valid`
      (if (`KismetArrayLibrary.Array_Contains` (`self.PickupsInRange`) _returnvalue)
        (`KismetArrayLibrary.Array_RemoveItem` (`self.PickupsInRange`) _returnvalue)
        (set `/Game/_Game/Blueprints/BPA_Pickup.IsSelected` false _returnvalue)))))

(fn `ClosestPickup`
  (locals (MaxDot :type "Float (double-precision)") (CurrentDot :type "Float (double-precision)" :default 0.0) (MinDotIndex :type Integer) (CurrentIndex :type Integer) (MinPickup :type "/Game/_Game/Blueprints/BPA_Pickup Object Reference") (CurrentPickup :type "/Game/_Game/Blueprints/BPA_Pickup Object Reference"))
  (bind _minpickup (`local.MinPickup`))
  (if (> (`KismetArrayLibrary.Array_Length` (`self.PickupsInRange`)) 0)
    (set `local.CurrentIndex` -1)
    (set `local.MaxDot` 0.0)
    (for _array_element (`self.PickupsInRange`)
      (bind _output_get (set `local.CurrentPickup` _array_element))
      (set `/Game/_Game/Blueprints/BPA_Pickup.IsSelected` false _output_get)
      (bind _output_get_2 (set `local.CurrentDot` (`KismetMathLibrary.Dot_VectorVector` (`KismetMathLibrary.Normal` (- (`self.K2_GetActorLocation` (`ActorComponent.GetOwner` _array_element)) (`self.K2_GetActorLocation`))) (`KismetMathLibrary.Normal` (`self.RotationDirection`)))))
      (if (>= _output_get_2 0.6)
        (if (> (`local.CurrentDot`) (`local.MaxDot`))
          (set `local.MinPickup` (`local.CurrentPickup`)))))
    (`/Engine/EditorBlueprintResources/StandardMacros.IsValid` (`local.MinPickup`)
      (:`Is Valid`
        (`KismetSystemLibrary.DrawDebugLine` (`self.K2_GetActorLocation`) (`self.K2_GetActorLocation` (`ActorComponent.GetOwner` (`local.MinPickup`))) (struct :`R` 0.635417 :`G` 0.555946 :`A` 1.0) 0.0 4.0)
        (set `self.SelectedPickup` _minpickup)
        (set `/Game/_Game/Blueprints/BPA_Pickup.IsSelected` true _minpickup)))
    (else
      (return))))

(fn `SetTargetR`
  (params (Position :type "Vector Structure")))

(fn `UserConstructionScript`)
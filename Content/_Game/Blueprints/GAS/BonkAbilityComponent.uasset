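; BonkAbilityComponent is a component that holds an actor's BonkPlayerData and its list of effects, in a lightweight custom ability setup.
; On BeginPlay it constructs and initializes the PlayerData object, which GetData exposes.
; AddEffect constructs an effect from a class, activates it against that PlayerData and appends it to the Effects array.
; Nothing here removes or updates effects.
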(event `self.ReceiveBeginPlay`
  ;[1 1 1] Construct player data
  (bind _returnvalue (`|GenericCreateObject` "/Game/_Game/Blueprints/GAS/BonkPlayerData.BonkPlayerData_C"))
  (bind _output_get (set `self.PlayerData` _returnvalue))
  (`/Game/_Game/Blueprints/GAS/BonkPlayerData.Init` _output_get))

(fn `AddEffect`
  (params (EffectClass :type "/Game/_Game/Blueprints/GAS/Effects/BonkEffect Class Reference"))
  (bind _returnvalue (`|GenericCreateObject` EffectClass))
  (`/Game/_Game/Blueprints/GAS/Effects/BonkEffect.OnActivate` _returnvalue (`self.PlayerData`))
  (`KismetArrayLibrary.Array_Add` (`self.Effects`) _returnvalue))

(fn `GetData`
  (returns (PlayerData :type "/Game/_Game/Blueprints/GAS/BonkPlayerData Object Reference"))
  (return (`self.PlayerData`)))
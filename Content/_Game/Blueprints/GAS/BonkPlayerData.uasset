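; BonkPlayerData is a player data container that holds Health and Damage attributes for the Bonk attribute system.
; Init constructs and initializes one attribute object for each.
; GetAttributeOfClass returns the attribute whose class exactly matches the requested one, along with a Found flag, using a hard-coded check per attribute.
; LogData prints both current values for debugging.
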(fn `GetAttributeOfClass`
  (params (AttributeClass :type "/Game/_Game/Blueprints/GAS/Attributes/BonkAttribute Class Reference"))
  (returns (AttributeRef :type "/Game/_Game/Blueprints/GAS/Attributes/BonkAttribute Object Reference") (`Found?` :type Boolean))
  (locals (LocalAttribClass :type "/Game/_Game/Blueprints/GAS/Attributes/BonkAttribute Class Reference") (FoundFlag :type Boolean))
  (set `local.LocalAttribClass` AttributeClass)
  (`|ExecutionSequence`
    (:`then_0`
      (if (== (`local.LocalAttribClass`) (`GameplayStatics.GetObjectClass` (`self.Health`)))
        (return (`self.Health`) true)))
    (:`then_1`
      (if (== (`local.LocalAttribClass`) (`GameplayStatics.GetObjectClass` (`self.Damage`)))
        (return (`self.Damage`) true)))
    (:`then_2`
      (return null false))))

(fn `Init`
  ;[1 1 1] Initialize attributes
  (bind _returnvalue (`|GenericCreateObject` "/Game/_Game/Blueprints/GAS/Attributes/BonkAttribute_Health.BonkAttribute_Health_C"))
  (bind _output_get (set `self.Health` _returnvalue))
  (`/Game/_Game/Blueprints/GAS/Attributes/BonkAttribute.Init` _output_get)
  (bind _returnvalue_2 (`|GenericCreateObject` "/Game/_Game/Blueprints/GAS/Attributes/BonkAttribute_Damage.BonkAttribute_Damage_C"))
  (bind _output_get_2 (set `self.Damage` _returnvalue_2))
  (`/Game/_Game/Blueprints/GAS/Attributes/BonkAttribute.Init` _output_get_2))

(fn `LogData`
  (`KismetSystemLibrary.PrintString` null (`KismetStringLibrary.Concat_StrStr` "Health: " (`KismetStringLibrary.Conv_DoubleToString` (`/Game/_Game/Blueprints/GAS/Attributes/BonkAttribute.CurrentValue` (`self.Health`)))))
  (`KismetSystemLibrary.PrintString` null (`KismetStringLibrary.Concat_StrStr` "Damage: " (`KismetStringLibrary.Conv_DoubleToString` (`/Game/_Game/Blueprints/GAS/Attributes/BonkAttribute.CurrentValue` (`self.Damage`))))))
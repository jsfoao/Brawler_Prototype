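; BPA_Damageable is a damageable Blueprint that tracks health and reports it to a health bar widget.
; Health starts at MaxHealth on BeginPlay, and TakeDamage subtracts the incoming damage without clamping or handling death.
; TakeDamage then casts WidgetRef to UMG_HealthBar and sets its percent to the ratio of current to maximum health.
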(event `self.ReceiveBeginPlay`
  (set `self.Health` (`self.MaxHealth`)))

(fn `TakeDamage`
  (params (Damage :type Integer))
  (bind _output_get (set `self.Health` (- (`self.Health`) Damage)))
  (bind _asumg_health_bar (cast `/Game/_Game/UI/UMG_HealthBar` (`self.WidgetRef`)))
  (`/Game/_Game/UI/UMG_HealthBar.SetPercent` _asumg_health_bar (/ (`KismetMathLibrary.Conv_IntToDouble` _output_get) (`KismetMathLibrary.Conv_IntToDouble` (`self.MaxHealth`)))))
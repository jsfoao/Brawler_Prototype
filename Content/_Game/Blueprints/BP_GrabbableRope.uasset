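; BP_GrabbableRope is a rope that a player can be attached to and released from, pairing a visual cable with a physics constraint.
; AttachPlayer pins the cable's end to the given actor and constrains StaticMesh to the passed primitive component.
; DetachPlayer frees the cable's end and re-targets the constraint from the player to StaticMesh1, so the constraint is swapped rather than broken.
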(event `self.DetachPlayer`
  (set `CableComponent.bAttachEnd` false (`self.Rope`)) ; Detach the visual cable
  (`PhysicsConstraintComponent.SetConstrainedComponents` (`self.PhysicsConstraint`) (`self.StaticMesh`) "None" (`self.StaticMesh1`) "None") ; Remove player from constraint
)

(event `self.AttachPlayer`
  (params (Actor :type "Actor Object Reference") (PrimitiveComponent :type "PrimitiveComponent Object Reference"))
  (bind _rope (`self.Rope`))
  ;[1 1 1] Attach the visual cable to player
  (`CableComponent.SetAttachEndTo` _rope Actor "None" "None")
  (set `CableComponent.bAttachEnd` true _rope)
  (set `CableComponent.EndLocation` (0.0 0.0 0.0) _rope)
  (`PhysicsConstraintComponent.SetConstrainedComponents` (`self.PhysicsConstraint`) (`self.StaticMesh`) "None" PrimitiveComponent "None") ; Constrain player
)

(fn `UserConstructionScript`)
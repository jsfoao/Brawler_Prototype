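; Sword pickup that acts as a melee weapon while an agent holds it and is attacking.
; Each tick it sphere-traces along the blade from the handle, ignoring the holder and drawing debug shapes.
; Damageable hits go to BPAPickup's OnHit, while hits on other pickups call its own OnGetHit.
; An OnHit flag blocks further traces, clearing after a short delay only in those two cases.
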(event `self.ReceiveTick`
  (params (DeltaSeconds :type "Float (single-precision)"))
  (bind _returnvalue (`SceneComponent.K2_GetComponentLocation` (`self.Handle`)))
  (bind _heldbyagent (`/Game/_Game/Blueprints/Components/BPA_Pickup.HeldByAgent` (`self.BPA_Pickup`)))
  (if (not (`self.OnHit`))
    (`/Engine/EditorBlueprintResources/StandardMacros.IsValid` _heldbyagent
      (:`Is Valid`
        (if (`/Game/_Game/Blueprints/Components/BPA_Pickup.IsAttacking` (`self.BPA_Pickup`))
          (bind (_outhits _returnvalue_2) (`KismetSystemLibrary.SphereTraceMultiForObjects` _returnvalue (+ _returnvalue (* (`self.GetActorUpVector`) 100.0)) 15.0 (`|MakeArray` "ObjectTypeQuery3" "ObjectTypeQuery7" :!type "EObjectTypeQuery Enum") false (`|MakeArray` (`ActorComponent.GetOwner` _heldbyagent)) "ForOneFrame" true (struct :`R` 1.0 :`A` 1.0) (struct :`G` 1.0 :`A` 1.0) 0.0))
          (if _returnvalue_2
            (set `self.OnHit` true)
            (for _array_element _outhits
              (bind (_bblockinghit _binitialoverlap _time _distance _location _impactpoint _normal _impactnormal _physmat _hitactor) (`GameplayStatics.BreakHitResult` _array_element))
              (`KismetSystemLibrary.DrawDebugSphere` _location 15.0 12 (struct :`R` 1.0 :`A` 1.0) 2.0 2.0)
              (bind _returnvalue_3 (`self.GetComponentByClass` _hitactor "/Game/_Game/Blueprints/Components/BPA_Damageable.BPA_Damageable_C"))
              (`/Engine/EditorBlueprintResources/StandardMacros.IsValid` _returnvalue_3
                (:`Is Valid`
                  (`/Game/_Game/Blueprints/Components/BPA_Pickup.OnHit` (`self.BPA_Pickup`) _returnvalue_3 _array_element))
                (:`Is Not Valid`
                  (`/Engine/EditorBlueprintResources/StandardMacros.IsValid` (`self.GetComponentByClass` _hitactor "/Game/_Game/Blueprints/Components/BPA_Pickup.BPA_Pickup_C")
                    (:`Is Valid`
                      (`/Game/_Game/Blueprints/Components/BPA_Pickup.OnGetHit` (`self.BPA_Pickup`))))))
              (`KismetSystemLibrary.Delay` 0.3)
              (set `self.OnHit` false))))))))

(fn `UserConstructionScript`
  (`parent.UserConstructionScript`))
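; Player character with camera-relative movement, mouse or gamepad aiming, and independent two-handed item use.
; BPPickupAgent grabs the pickup selected by a facing dot-product test among those in overlap range, and throws it with force charged while holding the button.
; Depending on held item type, each hand attacks or blocks through timelines that offset its transform from cached defaults.
; Blocking halves walk speed and prevents attacks.
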(event `self.ReceiveBeginPlay`
  ;[1 1 1] Inital setup
  (bind _returnvalue (`GameplayStatics.GetActorOfClass` "/Game/_Game/Blueprints/Actors/BP_FollowCamera.BP_FollowCamera_C"))
  (set `self.FollowCam` _returnvalue)
  (bind _output_get (set `self.Default_R` (`SceneComponent.GetRelativeTransform` (`self.Hand_R`))))
  (set `self.Default_R_Block` (`KismetMathLibrary.MakeTransform` (.location _output_get) (`KismetMathLibrary.MakeRotator` (.roll (.rotation _output_get)) 90.0 70.0) (.scale _output_get)))
  (bind _output_get_2 (set `self.Default_L` (`SceneComponent.GetRelativeTransform` (`self.Hand_L`))))
  (set `self.Default_L_Block` (`KismetMathLibrary.MakeTransform` (.location _output_get_2) (`KismetMathLibrary.MakeRotator` (.roll (.rotation _output_get_2)) 90.0 -70.0) (.scale _output_get_2)))
  (set `self.CanAttackRight` true)
  (set `CharacterMovementComponent.MaxWalkSpeed` (`self.MoveSpeed`) (`self.CharacterMovement`))
  (set `self.RotationDirection` (`KismetMathLibrary.Normal` (`self.GetActorForwardVector`)))
  (`/Game/_Game/Blueprints/Components/BPA_PickupAgent.SetHands` (`self.BP_PickupAgent`) (`self.Hand_R`) (`self.Hand_L`)))

(event `InputAction|ThrowLeft`
  (params (Key :type "Key Structure"))
  (bind (_default_l_block_location _default_l_block_rotation) (`KismetMathLibrary.BreakTransform` (`self.Default_L_Block`)))
  (bind (_default_l_location _default_l_rotation) (`KismetMathLibrary.BreakTransform` (`self.Default_L`)))
  ;[1 1 1] Throw/Pickup Left
  (:`Pressed`
    (`/Engine/EditorBlueprintResources/StandardMacros.IsValid` (`/Game/_Game/Blueprints/Components/BPA_PickupAgent.ObjectLeft` (`self.BP_PickupAgent`))
      (:`Is Valid`
        (set `self.ThrowLeftPressed` true))
      (:`Is Not Valid`
        (`/Game/_Game/Blueprints/Components/BPA_PickupAgent.PickupLeft` (`self.BP_PickupAgent`))
        (set `/Game/_Game/Blueprints/Components/BPA_PickupAgent.LeftGrabbedFrame` true (`self.BP_PickupAgent`))
        (bind _objectleft (`/Game/_Game/Blueprints/Components/BPA_PickupAgent.ObjectLeft` (`self.BP_PickupAgent`))
          (:`then`
            (if (`|EnumEquality` (`/Game/_Game/Blueprints/Components/BPA_Pickup.Type` _objectleft) "NewEnumerator0")
              (`SceneComponent.K2_SetRelativeRotation` (`self.Hand_L`) _default_l_block_rotation false false)))
          (:`else`)))))
  (:`Released`
    (if (`/Game/_Game/Blueprints/Components/BPA_PickupAgent.LeftGrabbedFrame` (`self.BP_PickupAgent`))
      (set `/Game/_Game/Blueprints/Components/BPA_PickupAgent.LeftGrabbedFrame` false (`self.BP_PickupAgent`))
      (else
        (set `self.ThrowLeftPressed` false)
        (`/Game/_Game/Blueprints/Components/BPA_PickupAgent.DropLeft` (`self.BP_PickupAgent`) (* (`self.RotationDirection`) (`self.ThrowMeterL`)))
        (`SceneComponent.K2_SetRelativeRotation` (`self.Hand_L`) _default_l_rotation false false)))))

(event `InputAction|ThrowRight`
  (params (Key :type "Key Structure"))
  (bind (_default_r_location _default_r_rotation) (`KismetMathLibrary.BreakTransform` (`self.Default_R`)))
  (bind (_default_r_block_location _default_r_block_rotation) (`KismetMathLibrary.BreakTransform` (`self.Default_R_Block`)))
  ;[1 1 1] Throw/Pickup Right
  (:`Pressed`
    (`/Engine/EditorBlueprintResources/StandardMacros.IsValid` (`/Game/_Game/Blueprints/Components/BPA_PickupAgent.ObjectRight` (`self.BP_PickupAgent`))
      (:`Is Valid`
        (set `self.ThrowRightPressed` true))
      (:`Is Not Valid`
        (`/Game/_Game/Blueprints/Components/BPA_PickupAgent.PickupRight` (`self.BP_PickupAgent`))
        (set `/Game/_Game/Blueprints/Components/BPA_PickupAgent.RightGrabbedFrame` true (`self.BP_PickupAgent`))
        (bind _objectright (`/Game/_Game/Blueprints/Components/BPA_PickupAgent.ObjectRight` (`self.BP_PickupAgent`))
          (:`then`
            (if (`|EnumEquality` (`/Game/_Game/Blueprints/Components/BPA_Pickup.Type` _objectright) "NewEnumerator0")
              (`SceneComponent.K2_SetRelativeRotation` (`self.Hand_R`) _default_r_block_rotation false false)))
          (:`else`)))))
  (:`Released`
    (if (`/Game/_Game/Blueprints/Components/BPA_PickupAgent.RightGrabbedFrame` (`self.BP_PickupAgent`))
      (set `/Game/_Game/Blueprints/Components/BPA_PickupAgent.RightGrabbedFrame` false (`self.BP_PickupAgent`))
      (else
        (set `self.ThrowRightPressed` false)
        (`/Game/_Game/Blueprints/Components/BPA_PickupAgent.DropRight` (`self.BP_PickupAgent`) (* (`self.RotationDirection`) (`self.ThrowMeterR`)))
        (`SceneComponent.K2_SetRelativeRotation` (`self.Hand_R`) _default_r_rotation false false)))))

(event `InputAxis|Move Right / Left`
  (params (AxisValue :type "Float (single-precision)"))
  (bind _returnvalue (`self.GetActorRightVector` (`self.FollowCam`)))
  ;[1 1 1] Locomotion
  (`self.AddMovementInput` _returnvalue AxisValue)
  (set `self.MoveRightVec` (* _returnvalue AxisValue)))

(event `InputAxis|Move Forward / Backward`
  (params (AxisValue :type "Float (single-precision)"))
  (bind _returnvalue (`self.GetActorForwardVector` (`self.FollowCam`)))
  ;[1 1 1] Locomotion
  (`self.AddMovementInput` _returnvalue AxisValue)
  (set `self.MoveLeftVec` (* _returnvalue AxisValue)))

(event `InputAxis|Turn Right / Left Mouse`
  (params (AxisValue :type "Float (single-precision)"))
  ;[1 1 1] Locomotion
  (set `self.RotationDirection` (`KismetMathLibrary.RotateAngleAxis` (`self.RotationDirection`) (* AxisValue (`self.RotationSpeed`)) (0.0 0.0 1.0))))

(event `InputAxis|Turn Right / Left Gamepad`
  (params (AxisValue :type "Float (single-precision)"))
  ;[1 1 1] Locomotion
  ;;[1 1 1] Gamepad rotation
  (set `self.RightDir` (* AxisValue (`self.GetActorRightVector` (`self.FollowCam`)))))

(event `InputAxis|Look Up / Down Gamepad`
  (params (AxisValue :type "Float (single-precision)"))
  ;[1 1 1] Locomotion
  ;;[1 1 1] Gamepad rotation
  (set `self.LeftDir` (* AxisValue (`self.GetActorForwardVector` (`self.FollowCam`)) -1.0)))

(event `InputAction|AttackRight`
  (params (Key :type "Key Structure"))
  ;[1 1 1] Combat
  (:`Pressed`
    (bind _objectright (`/Game/_Game/Blueprints/Components/BPA_PickupAgent.ObjectRight` (`self.BP_PickupAgent`))
      (:`then`
        (if (`|EnumEquality` (`/Game/_Game/Blueprints/Components/BPA_Pickup.Type` _objectright) "NewEnumerator1")
          (if (or (`self.IsBlockingRight`) (`self.IsBlockingLeft`))
            _
            (elif (`self.CanAttackRight`)
              (set `self.IsAttackingRight` true)
              (set `self.CanAttackRight` false)
              (set `/Game/_Game/Blueprints/Components/BPA_Pickup.IsAttacking` true (`/Game/_Game/Blueprints/Components/BPA_PickupAgent.ObjectRight` (`self.BP_PickupAgent`)))
              (bind (_direction _translation _rotation) (`Timeline|AttackR_Timeline` :!via `PlayFromStart`)
                (:`Update`
                  (`self.AddLocRotRightHand` _translation _rotation (`self.Default_R`)))
                (:`Finished`
                  (set `self.CanAttackRight` true)
                  (set `self.IsAttackingRight` false)
                  (set `/Game/_Game/Blueprints/Components/BPA_Pickup.IsAttacking` false (`/Game/_Game/Blueprints/Components/BPA_PickupAgent.ObjectRight` (`self.BP_PickupAgent`)))))))
          (else
            (set `self.IsBlockingRight` true)
            (bind (_direction_2 _translation_2 _rotation_2) (`Timeline|BlockR_Timeline` :!label _label)
              (:`Update`
                (`self.AddLocRotRightHand` _translation_2 _rotation_2 (`self.Default_R_Block`)))))))
      (:`else`)))
  (:`Released`
    (bind _objectright_2 (`/Game/_Game/Blueprints/Components/BPA_PickupAgent.ObjectRight` (`self.BP_PickupAgent`))
      (:`then`
        (if (`|EnumEquality` (`/Game/_Game/Blueprints/Components/BPA_Pickup.Type` _objectright_2) "NewEnumerator0")
          (set `self.IsBlockingRight` false)
          (goto _label :!via `Reverse`)))
      (:`else`))))

(event `InputAction|AttackLeft`
  (params (Key :type "Key Structure"))
  ;[1 1 1] Combat
  (:`Pressed`
    (bind _objectleft (`/Game/_Game/Blueprints/Components/BPA_PickupAgent.ObjectLeft` (`self.BP_PickupAgent`))
      (:`then`
        (if (`|EnumEquality` (`/Game/_Game/Blueprints/Components/BPA_Pickup.Type` _objectleft) "NewEnumerator1")
          (if (or (`self.IsBlockingRight`) (`self.IsBlockingLeft`))
            _
            (elif (`self.CanAttackLeft`)
              (set `self.IsAttackingLeft` true)
              (set `self.CanAttackLeft` false)
              (set `/Game/_Game/Blueprints/Components/BPA_Pickup.IsAttacking` true (`/Game/_Game/Blueprints/Components/BPA_PickupAgent.ObjectLeft` (`self.BP_PickupAgent`)))
              (bind (_direction _translation _rotation) (`Timeline|AttackL_Timeline` :!via `PlayFromStart`)
                (:`Update`
                  (`self.AddLockRotLeftHand` _translation _rotation (`self.Default_L`)))
                (:`Finished`
                  (set `self.CanAttackLeft` true)
                  (set `self.IsAttackingLeft` false)
                  (set `/Game/_Game/Blueprints/Components/BPA_Pickup.IsAttacking` false (`/Game/_Game/Blueprints/Components/BPA_PickupAgent.ObjectLeft` (`self.BP_PickupAgent`)))))))
          (else
            (set `self.IsBlockingLeft` true)
            (bind (_direction_2 _translation_2 _rotation_2) (`Timeline|BlockL_Timeline` :!label _label_2)
              (:`Update`
                (`self.AddLockRotLeftHand` _translation_2 _rotation_2 (`self.Default_L_Block`)))))))
      (:`else`)))
  (:`Released`
    (bind _objectleft_2 (`/Game/_Game/Blueprints/Components/BPA_PickupAgent.ObjectLeft` (`self.BP_PickupAgent`))
      (:`then`
        (if (`|EnumEquality` (`/Game/_Game/Blueprints/Components/BPA_Pickup.Type` _objectleft_2) "NewEnumerator0")
          (set `self.IsBlockingLeft` false)
          (goto _label_2 :!via `Reverse`)))
      (:`else`))))

(event `self.ReceiveTick`
  (params (DeltaSeconds :type "Float (single-precision)"))
  (bind _returnvalue (`self.K2_GetActorLocation`))
  (bind _returnvalue_2 (`self.K2_GetActorLocation`))
  (bind _returnvalue_3 (`self.K2_GetActorLocation`))
  (bind _returnvalue_4 (`self.K2_GetActorLocation`))
  (bind (_returnvalue_roll _returnvalue_pitch _returnvalue_yaw) (`KismetMathLibrary.BreakRotator` (`KismetMathLibrary.RInterpTo` (`self.CurrentRotation`) (`KismetMathLibrary.FindLookAtRotation` (`KismetMathLibrary.Vector_Zero`) (`self.RotationDirection`)) (`GameplayStatics.GetWorldDeltaSeconds`) 5.0)))
  (bind (_returnvalue_x _returnvalue_y) (`KismetMathLibrary.BreakVector` (+ _returnvalue_2 (* (`KismetMathLibrary.Normal` (`self.RotationDirection`)) 100.0))))
  (`|ExecutionSequence`
    (:`then_0`
      (if (`self.Debug`)
        (`KismetSystemLibrary.DrawDebugLine` _returnvalue_2 (`KismetMathLibrary.MakeVector` _returnvalue_x _returnvalue_y (`.Z` (`KismetMathLibrary.BreakVector3f` _returnvalue_2))) (struct :`R` 1.0 :`A` 1.0) 0.0 4.0)
        (`/Game/_Game/Blueprints/BP_UtilityLib.LogBool` "IsBlockingRight" (`self.IsBlockingRight`))
        (`/Game/_Game/Blueprints/BP_UtilityLib.LogBool` "IsBlockingLeft" (`self.IsBlockingLeft`))
        (`/Game/_Game/Blueprints/BP_UtilityLib.LogBool` "CanAttack" (`self.CanAttackRight`))
        (`/Game/_Game/Blueprints/BP_UtilityLib.LogVec` "MovementInput" (`self.MovementInput`))
        (`/Game/_Game/Blueprints/BP_UtilityLib.LogVec` "RotationDirection" (`self.RotationDirection`))
        (`KismetSystemLibrary.DrawDebugLine` _returnvalue_4 (+ _returnvalue_4 (* (`KismetMathLibrary.Normal` (`self.MovementInput`)) 75.0)) (struct :`B` 1.0 :`A` 1.0) 0.0 4.0)
        (`KismetSystemLibrary.DrawDebugLine` (+ _returnvalue_3 (0.0 0.0 2.0)) (+ (+ _returnvalue_3 (* (`self.RotationDirection`) (`self.ThrowMeterR`) 100.0)) (0.0 0.0 2.0)) (struct :`G` 0.870588 :`B` 1.0 :`A` 1.0) 0.0 6.0)
        (`/Game/_Game/Blueprints/BP_UtilityLib.LogString` "SelectedPickup" (`KismetSystemLibrary.GetDisplayName` (`/Game/_Game/Blueprints/Components/BPA_PickupAgent.SelectedPickup` (`self.BP_PickupAgent`))))
        (`KismetSystemLibrary.DrawDebugLine` (+ _returnvalue (0.0 0.0 2.0)) (+ (+ _returnvalue (* (`self.RotationDirection`) (`self.ThrowMeterL`) 100.0)) (0.0 0.0 2.0)) (struct :`G` 0.870588 :`B` 1.0 :`A` 1.0) 0.0 6.0)))
    (:`then_1`
      (if (or (`self.IsBlockingRight`) (`self.IsBlockingLeft`))
        (set `CharacterMovementComponent.MaxWalkSpeed` (* (`self.MoveSpeed`) 0.5) (`self.CharacterMovement`))
        (else
          (set `CharacterMovementComponent.MaxWalkSpeed` (`self.MoveSpeed`) (`self.CharacterMovement`)))))
    (:`then_2`
      ;[1 1 1] Character Rotation
      (set `self.MovementInput` (+ (`self.MoveRightVec`) (`self.MoveLeftVec`)))
      (bind _output_get (set `self.RotationInput` (+ (`self.LeftDir`) (`self.RightDir`))))
      (if (> (`KismetMathLibrary.VSize` _output_get) 0.0)
        (set `self.RotationDirection` (`self.RotationInput`)))
      (bind _output_get_2 (set `self.CurrentRotation` (`KismetMathLibrary.MakeRotator` 0.0 0.0 _returnvalue_yaw)))
      (`self.K2_SetActorRotation` (`KismetMathLibrary.MakeRotator` 0.0 0.0 (.yaw _output_get_2))))
    (:`then_3`
      (`self.ClosestPickup`)
      (`self.RightMeter`)
      (`self.LeftMeter`))))

(event `self.PickupRange.OnComponentBeginOverlap`
  (params (OverlappedComponent :type "PrimitiveComponent Object Reference") (OtherActor :type "Actor Object Reference") (OtherComp :type "PrimitiveComponent Object Reference") (OtherBodyIndex :type Integer) (bFromSweep :type Boolean) (SweepResult :type "HitResult Structure (by ref)"))
  (bind _returnvalue (`self.GetComponentByClass` OtherActor "/Game/_Game/Blueprints/Components/BPA_Pickup.BPA_Pickup_C"))
  ;[1 1 1] Pickup range
  (`/Engine/EditorBlueprintResources/StandardMacros.IsValid` _returnvalue
    (:`Is Valid`
      (`KismetArrayLibrary.Array_AddUnique` (`self.PickupsInRange`) _returnvalue))))

(event `self.PickupRange.OnComponentEndOverlap`
  (params (OverlappedComponent :type "PrimitiveComponent Object Reference") (OtherActor :type "Actor Object Reference") (OtherComp :type "PrimitiveComponent Object Reference") (OtherBodyIndex :type Integer))
  (bind _returnvalue (`self.GetComponentByClass` OtherActor "/Game/_Game/Blueprints/Components/BPA_Pickup.BPA_Pickup_C"))
  ;[1 1 1] Pickup range
  (`/Engine/EditorBlueprintResources/StandardMacros.IsValid` _returnvalue
    (:`Is Valid`
      (if (`KismetArrayLibrary.Array_Contains` (`self.PickupsInRange`) _returnvalue)
        (`KismetArrayLibrary.Array_RemoveItem` (`self.PickupsInRange`) _returnvalue)
        (set `/Game/_Game/Blueprints/Components/BPA_Pickup.IsSelected` false _returnvalue)
        (set `/Game/_Game/Blueprints/Components/BPA_PickupAgent.SelectedPickup` null (`self.BP_PickupAgent`))))))

(event `self.CapsuleComponent.OnComponentHit`
  (params (HitComponent :type "PrimitiveComponent Object Reference") (OtherActor :type "Actor Object Reference") (OtherComp :type "PrimitiveComponent Object Reference") (NormalImpulse :type "Vector Structure") (Hit :type "HitResult Structure (by ref)")))

(fn `AddLockRotLeftHand`
  (params (Offset :type "Vector Structure") (Rotation :type "Vector3f Structure") (Default :type "Transform Structure (by ref)"))
  (bind (_x _y _z) (`KismetMathLibrary.BreakVector3f` Rotation))
  (`SceneComponent.K2_SetRelativeLocationAndRotation` (`self.Hand_L`) (+ Offset (.location Default)) (`KismetMathLibrary.ComposeRotators` (`KismetMathLibrary.MakeRotator` _x _y _z) (.rotation Default)) false false))

(fn `AddLocRotRightHand`
  (params (Offset :type "Vector Structure") (Rotation :type "Vector3f Structure") (Default :type "Transform Structure (by ref)"))
  (bind (_x _y _z) (`KismetMathLibrary.BreakVector3f` Rotation))
  (`SceneComponent.K2_SetRelativeLocationAndRotation` (`self.Hand_R`) (+ Offset (.location Default)) (`KismetMathLibrary.ComposeRotators` (`KismetMathLibrary.MakeRotator` _x _y _z) (.rotation Default)) false false))

(fn `ClosestPickup`
  (locals (MaxDot :type "Float (double-precision)") (CurrentDot :type "Float (double-precision)" :default 0.0) (MinDotIndex :type Integer) (CurrentIndex :type Integer) (MinPickup :type "/Game/_Game/Blueprints/Components/BPA_Pickup Object Reference") (CurrentPickup :type "/Game/_Game/Blueprints/Components/BPA_Pickup Object Reference"))
  (bind _minpickup (`local.MinPickup`))
  (if (> (`KismetArrayLibrary.Array_Length` (`self.PickupsInRange`)) 0)
    (set `local.CurrentIndex` -1)
    (set `local.MaxDot` 0.0)
    (for _array_element (`self.PickupsInRange`)
      (bind _output_get (set `local.CurrentPickup` _array_element))
      (set `/Game/_Game/Blueprints/Components/BPA_Pickup.IsSelected` false _output_get)
      (bind _output_get_2 (set `local.CurrentDot` (`KismetMathLibrary.Dot_VectorVector` (`KismetMathLibrary.Normal` (- (`self.K2_GetActorLocation` (`ActorComponent.GetOwner` _array_element)) (`self.K2_GetActorLocation`))) (`KismetMathLibrary.Normal` (`self.RotationDirection`)))))
      (if (>= _output_get_2 0.6)
        (if (> (`local.CurrentDot`) (`local.MaxDot`))
          (set `local.MinPickup` (`local.CurrentPickup`)))))
    (`/Engine/EditorBlueprintResources/StandardMacros.IsValid` (`local.MinPickup`)
      (:`Is Valid`
        (`KismetSystemLibrary.DrawDebugLine` (`self.K2_GetActorLocation`) (`self.K2_GetActorLocation` (`ActorComponent.GetOwner` (`local.MinPickup`))) (struct :`R` 0.635417 :`G` 0.555946 :`A` 1.0) 0.0 4.0)
        (set `/Game/_Game/Blueprints/Components/BPA_PickupAgent.SelectedPickup` _minpickup (`self.BP_PickupAgent`))
        (set `/Game/_Game/Blueprints/Components/BPA_Pickup.IsSelected` true _minpickup))
      (:`Is Not Valid`
        (set `/Game/_Game/Blueprints/Components/BPA_PickupAgent.SelectedPickup` null (`self.BP_PickupAgent`))))
    (else
      (return))))

(fn `LeftMeter`
  (if (`self.ThrowLeftPressed`)
    (bind _output_get (set `self.ThrowMeterL` (`KismetMathLibrary.FClamp` (+ (`self.ThrowMeterL`) (`GameplayStatics.GetWorldDeltaSeconds`)))))
    (`/Game/_Game/Blueprints/BP_UtilityLib.LogFloat` "ThrowL" _output_get)
    (else
      (bind _output_get_2 (set `self.ThrowMeterL` 0.0))
      (`/Game/_Game/Blueprints/BP_UtilityLib.LogFloat` "ThrowL" _output_get_2))))

(fn `RightMeter`
  (if (`self.ThrowRightPressed`)
    (set `self.ThrowMeterR` (`KismetMathLibrary.FClamp` (+ (`self.ThrowMeterR`) (`GameplayStatics.GetWorldDeltaSeconds`))))
    (else
      (set `self.ThrowMeterR` 0.0))))

(fn `SetTargetR`
  (params (Position :type "Vector Structure")))

(fn `UserConstructionScript`)
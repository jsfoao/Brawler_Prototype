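; BP_Cannon is a mounted weapon actor that turns toward an aim direction and fires physics-driven projectiles.
; HandleRotation smoothly interpolates toward the given direction and applies only the yaw to the whole actor.
; Shoot calls the parent, then, if mounted and ready, spawns a BP_Projectile at the Arrow component and launches its mesh with a forward impulse.
; A CanShoot flag and a delay enforce the cooldown between shots.
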(event `self.HandleRotation`
  (params (RotationDirection :type "Vector Structure"))
  (bind (_returnvalue_roll _returnvalue_pitch _returnvalue_yaw) (`KismetMathLibrary.BreakRotator` (`KismetMathLibrary.RInterpTo` (`self.CurrentRotation`) (`KismetMathLibrary.FindLookAtRotation` (`KismetMathLibrary.Vector_Zero`) RotationDirection) (`GameplayStatics.GetWorldDeltaSeconds`) 5.0)))
  (bind _output_get (set `self.CurrentRotation` (`KismetMathLibrary.MakeRotator` 0.0 0.0 _returnvalue_yaw)))
  (`self.K2_SetActorRotation` (`KismetMathLibrary.MakeRotator` 0.0 0.0 (.yaw _output_get))))

(event `self.Shoot`
  (`parent.Shoot`)
  (if (and (`self.IsMounted`) (`self.CanShoot`))
    (bind _returnvalue (`|SpawnActorFromClass` "/Game/_Game/Blueprints/Actors/MountedWeapons/BP_Projectile.BP_Projectile_C" (`SceneComponent.K2_GetComponentToWorld` (`self.Arrow`)) "Undefined" "OverrideRootScale" null null))
    (`PrimitiveComponent.AddImpulse` (`/Game/_Game/Blueprints/Actors/MountedWeapons/BP_Projectile.StaticMesh` _returnvalue) (* (`SceneComponent.GetForwardVector` (`self.Arrow`)) 50000.0) "None" false)
    (set `self.CanShoot` false)
    (`KismetSystemLibrary.Delay` (`self.ShootCooldown`))
    (set `self.CanShoot` true)))

(fn `UserConstructionScript`
  (`parent.UserConstructionScript`))
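; Mortar mounted weapon that slides along its forward axis, turns to aim and launches physics projectiles.
; Movement input teleports the Sphere component forward or back, while rotation input smoothly interpolates yaw toward the input direction.
; Shoot extends the parent event, spawning BP_Projectile at the Arrow with a velocity-change impulse when mounted, gated by a cooldown.
; BeginPlay automatically mounts and fires once after a short delay.
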(event `self.HandleMovement`
  (params (moveDirection :type "Vector Structure"))
  (`SceneComponent.K2_AddWorldOffset` (`self.Sphere`) (* (`self.GetActorForwardVector`) moveDirection_X) false true))

(event `self.HandleRotation`
  (params (RotationDirection :type "Vector Structure"))
  (bind (_returnvalue_roll _returnvalue_pitch _returnvalue_yaw) (`KismetMathLibrary.BreakRotator` (`KismetMathLibrary.RInterpTo` (`self.CurrentRotation`) (`KismetMathLibrary.FindLookAtRotation` (`KismetMathLibrary.Vector_Zero`) RotationDirection) (`GameplayStatics.GetWorldDeltaSeconds`) 5.0)))
  (bind _output_get (set `self.CurrentRotation` (`KismetMathLibrary.MakeRotator` 0.0 0.0 _returnvalue_yaw)))
  (`self.K2_SetActorRotation` (`KismetMathLibrary.MakeRotator` 0.0 0.0 (.yaw _output_get))))

(event `self.ReceiveBeginPlay`
  (`KismetSystemLibrary.Delay` 2.0)
  (`self.Mount`)
  (`self.Shoot`))

(event `self.Shoot`
  (`parent.Shoot`)
  (if (and (`self.IsMounted`) (`self.CanShoot`))
    (bind _returnvalue (`|SpawnActorFromClass` "/Game/_Game/Blueprints/Actors/MountedWeapons/BP_Projectile.BP_Projectile_C" (`SceneComponent.K2_GetComponentToWorld` (`self.Arrow`)) "Undefined" "OverrideRootScale" null null))
    (`PrimitiveComponent.AddImpulse` (`/Game/_Game/Blueprints/Actors/MountedWeapons/BP_Projectile.StaticMesh` _returnvalue) (* (`SceneComponent.GetForwardVector` (`self.Arrow`)) 1000.0) "None" true)
    (set `self.CanShoot` false)
    (`KismetSystemLibrary.Delay` (`self.ShootCooldown`))
    (set `self.CanShoot` true)))

(fn `UserConstructionScript`
  (`parent.UserConstructionScript`))
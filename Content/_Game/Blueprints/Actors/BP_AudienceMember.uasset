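; Audience member actor that bobs up and down continuously in a bouncing motion.
; Tick accumulates time and feeds the absolute value of a sine math expression into the world Z passed to SetActorLocation, without adding the starting height.
; BeginPlay caches an AudioVolume actor as Manager and records the starting height, but neither is used afterwards.
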(event EventBeginPlay
  (Utilities|FlowControl|Sequence
    (:then_0
      (bind _returnvalue (Actor|GetActorOfClass "/Script/Engine.AudioVolume"))
      (Variables|Default|SetManager _returnvalue))
    (:then_1
      (Variables|Default|SetStartHeight (.z (Transformation|GetActorLocation))))))

(event EventTick
  (params (DeltaSeconds :type Float%20%28single-precision%29))
  (Variables|Default|SetTime (+ DeltaSeconds (Variables|Default|GetTime)))
  (Transformation|SetActorLocation (Math|Vector|MakeVector 0.0 0.0 (Math|Float|Absolute(Float) (* (|(a*(sin((b*x)))) 1.0 1.0 (Variables|Default|GetTime)) 1e+02))) false false))

(fn ConstructionScript)
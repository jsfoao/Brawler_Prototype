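; BP_KillFloor is a rising lava hazard that kills damageable actors and removes pickups it touches.
; On BeginPlay it binds to the press event of the BP_Button in the level, and MoveLavaUp uses a timeline to lerp its height to TargetHeight.
; Mesh overlaps call OnDeath on BPA_Damageable components, otherwise passing BP_PickupTest owners of BPA_Pickup components to BP_SpawnManager's RemoveWeapon.
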(event `self.ReceiveBeginPlay`
  (bind _returnvalue (`GameplayStatics.GetActorOfClass` "/Game/_Game/Blueprints/Actors/BP_Button.BP_Button_C"))
  (add `/Game/_Game/Blueprints/Actors/BP_Button.OnButtonPress` _returnvalue (`|CreateDelegate` :!event `MoveLavaUp`)))

(event `MoveLavaUp`
  (bind (_startpos_x _startpos_y _startpos_z) (`KismetMathLibrary.BreakVector` (`self.StartPos`)))
  (set `self.StartPos` (`self.K2_GetActorLocation`))
  (bind (_direction _newtrack_0) (`Timeline|Lava` :!via `PlayFromStart`)
    (:`Update`
      (`self.K2_SetActorLocation` (`KismetMathLibrary.MakeVector` _startpos_x _startpos_y (`KismetMathLibrary.Lerp` _startpos_z (`self.target Height`) _newtrack_0))))))

(event `self.StaticMeshComponent.OnComponentBeginOverlap`
  (params (OverlappedComponent :type "PrimitiveComponent Object Reference") (OtherActor :type "Actor Object Reference") (OtherComp :type "PrimitiveComponent Object Reference") (OtherBodyIndex :type Integer) (bFromSweep :type Boolean) (SweepResult :type "HitResult Structure (by ref)"))
  (bind _returnvalue (`self.GetComponentByClass` OtherActor "/Game/_Game/Blueprints/Components/BPA_Damageable.BPA_Damageable_C"))
  (bind _returnvalue_2 (`self.GetComponentByClass` OtherActor "/Game/_Game/Blueprints/Components/BPA_Pickup.BPA_Pickup_C"))
  (`/Engine/EditorBlueprintResources/StandardMacros.IsValid` _returnvalue
    (:`Is Valid`
      (`/Game/_Game/Blueprints/Components/BPA_Damageable.OnDeath` _returnvalue))
    (:`Is Not Valid`
      (`/Engine/EditorBlueprintResources/StandardMacros.IsValid` _returnvalue_2
        (:`Is Valid`
          (bind _returnvalue_3 (`GameplayStatics.GetActorOfClass` "/Game/_Game/Blueprints/Actors/BP_SpawnManager.BP_SpawnManager_C"))
          (`/Engine/EditorBlueprintResources/StandardMacros.IsValid` _returnvalue_3
            (:`Is Valid`
              (bind _asbp_pickup_test (cast `/Game/_Game/Blueprints/Pickups/BP_PickupTest` (`ActorComponent.GetOwner` _returnvalue_2)))
              (`/Game/_Game/Blueprints/Actors/BP_SpawnManager.RemoveWeapon` _returnvalue_3 _asbp_pickup_test))))))))

(fn `UserConstructionScript`)
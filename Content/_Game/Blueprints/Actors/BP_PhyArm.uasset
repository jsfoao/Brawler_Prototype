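; BP_PhyArm is a physics-driven arm actor that punches toward a target actor, TargetR.
; Punch applies a force to ArmLowerR at the BoneHandR location along the normalized direction to the target, scaled by PunchMulti.
; Tick only draws a red debug line from hand to target.
; An unconnected variant with a distance-scaled pull toward the target remains in the event graph but never runs.
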(event `self.ReceiveTick`
  (params (DeltaSeconds :type "Float (single-precision)"))
  (`KismetSystemLibrary.DrawDebugLine` (`SceneComponent.K2_GetComponentLocation` (`self.Bone_Hand_R`)) (`self.K2_GetActorLocation` (`self.Target_R`)) (struct :`R` 1.0 :`A` 1.0) 0.0 3.0))

(fn `Punch`
  (`/Engine/EditorBlueprintResources/StandardMacros.IsValid` (`self.Target_R`)
    (:`Is Valid`
      (bind _output_get (set `self.DirectionVec` (`KismetMathLibrary.Normal` (- (`self.K2_GetActorLocation` (`self.Target_R`)) (`SceneComponent.K2_GetComponentLocation` (`self.Bone_Hand_R`))))))
      (`PrimitiveComponent.AddForceAtLocation` (`self.Arm_Lower_R`) (* _output_get (`self.PunchMulti`)) (`SceneComponent.K2_GetComponentLocation` (`self.Bone_Hand_R`)) "None"))))

(fn `UserConstructionScript`)
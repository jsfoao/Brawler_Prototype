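; BP_Button is a pushable button actor that fires an OnButtonPress event dispatcher when its Pressable component is pressed in.
; Tick compares the world Y positions of Scene and Pressable, treating a gap under 7 units as a press.
; A DoOnce with no reset limits the dispatcher and debug print to the first press.
; BeginPlay stores Pressable's starting Z, but the press check does not use it.
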(event `self.ReceiveBeginPlay`
  (bind (_returnvalue_x _returnvalue_y _returnvalue_z) (`KismetMathLibrary.BreakVector` (`SceneComponent.K2_GetComponentLocation` (`self.Pressable`))))
  (set `self.Start` _returnvalue_z))

(event `self.ReceiveTick`
  (params (DeltaSeconds :type "Float (single-precision)"))
  (bind (_returnvalue_x _returnvalue_y) (`KismetMathLibrary.BreakVector` (`SceneComponent.K2_GetComponentLocation` (`self.Scene`))))
  (bind (_returnvalue_x_2 _returnvalue_y_2) (`KismetMathLibrary.BreakVector` (`SceneComponent.K2_GetComponentLocation` (`self.Pressable`))))
  ;[1 1 1] Check if we are pressed in
  (if (< (`KismetMathLibrary.Abs` (- _returnvalue_y _returnvalue_y_2)) 7.0)
    (`/Engine/EditorBlueprintResources/StandardMacros.DoOnce` false
      (:`Completed`
        (`KismetSystemLibrary.PrintString` "Pressed")
        (`self.OnButtonPress`)))))

(fn `UserConstructionScript`)
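; BP_SpawnManager is an actor that keeps weapon pickups stocked in the level by tracking them in SpawnedPickups.
; BeginPlay fills the list with existing BP_PickupTest actors, and Tick spawns two weapons whenever it is empty.
; SpawnWeapon pairs a random WeaponPool class with a random SpawnPoints transform, though Length-1 as RandomInteger's max excludes each array's last entry.
; AddWeapon registers each spawn, and RemoveWeapon takes pickups off the list.
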(event `self.ReceiveBeginPlay`
  (bind _outactors (`GameplayStatics.GetAllActorsOfClass` "/Game/_Game/Blueprints/Pickups/BP_PickupTest.BP_PickupTest_C"))
  (set `self.SpawnedPickups` _outactors))

(event `self.ReceiveTick`
  (params (DeltaSeconds :type "Float (single-precision)"))
  (if (<= (`KismetArrayLibrary.Array_Length` (`self.SpawnedPickups`)) 0)
    (`self.SpawnWeapon`)
    (`self.SpawnWeapon`)))

(fn `AddWeapon`
  (params (PickupTest :type "/Game/_Game/Blueprints/Pickups/BP_PickupTest Object Reference (by ref)"))
  (`KismetArrayLibrary.Array_Add` (`self.SpawnedPickups`) PickupTest))

(fn `RemoveWeapon`
  (params (PickupTest :type "/Game/_Game/Blueprints/Pickups/BP_PickupTest Object Reference (by ref)"))
  (`KismetArrayLibrary.Array_RemoveItem` (`self.SpawnedPickups`) PickupTest))

(fn `SpawnWeapon`
  (bind _spawnpoints (`self.SpawnPoints`))
  (bind _weaponpool (`self.WeaponPool`))
  (bind _returnvalue (`|SpawnActorFromClass` (`|GetArrayItem` _weaponpool (`KismetMathLibrary.RandomInteger` (- (`KismetArrayLibrary.Array_Length` _weaponpool) 1))) (`|GetArrayItem` _spawnpoints (`KismetMathLibrary.RandomInteger` (- (`KismetArrayLibrary.Array_Length` _spawnpoints) 1))) "Undefined" "OverrideRootScale" null null))
  (`self.AddWeapon` _returnvalue))

(fn `UserConstructionScript`)
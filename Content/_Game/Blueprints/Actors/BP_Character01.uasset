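; BP_Character01 is a player character that moves relative to a BP_FollowCamera and throws punches with floating-offset hand components.
; Punch input picks a random hand and drives it from its default position with a timeline, blocking new punches until it finishes.
; While punching, overlaps on either hand's collision damage actors that have a BPA_Damageable component.
; Tick prints punch debug state; mouse turning and SetTargetR are unimplemented.
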(event `self.ReceiveBeginPlay`
  (bind _returnvalue (`GameplayStatics.GetActorOfClass` "/Game/_Game/Blueprints/Actors/BP_FollowCamera.BP_FollowCamera_C"))
  (set `self.FollowCam` _returnvalue)
  (set `self.Default_R` (`SceneComponent.RelativeLocation` (`self.Hand_R`)))
  (set `self.Default_L` (`SceneComponent.RelativeLocation` (`self.Hand_L`)))
  (set `self.CanPunch` true))

(event `InputAxis|Move Right / Left`
  (params (AxisValue :type "Float (single-precision)"))
  (`self.AddMovementInput` (* (* AxisValue (`self.GetActorRightVector` (`self.FollowCam`))) (`self.MoveSpeed`))))

(event `InputAxis|Move Forward / Backward`
  (params (AxisValue :type "Float (single-precision)"))
  (`self.AddMovementInput` (* (* AxisValue (`self.GetActorForwardVector` (`self.FollowCam`))) (`self.MoveSpeed`))))

(event `InputAxis|Turn Right / Left Mouse`
  (params (AxisValue :type "Float (single-precision)")))

(event `InputAction|Punch`
  (params (Key :type "Key Structure"))
  (:`Pressed`
    (if (`self.CanPunch`)
      (set `self.CanPunch` false)
      (set `self.IsPunching` true)
      (set `self.NextPunch` (`KismetMathLibrary.RandomBool`))
      (bind (_direction _offset) (`Timeline|Timeline_1` :!via `PlayFromStart`)
        (:`Update`
          (if (`self.NextPunch`)
            (`SceneComponent.K2_SetRelativeLocation` (`self.Hand_L`) (+ _offset (`self.Default_L`)) false false)
            (else
              (`SceneComponent.K2_SetRelativeLocation` (`self.Hand_R`) (+ _offset (`self.Default_R`)) false false))))
        (:`Finished`
          (set `self.CanPunch` true)
          (set `self.IsPunching` false))))))

(event `self.ReceiveTick`
  (params (DeltaSeconds :type "Float (single-precision)"))
  (`KismetSystemLibrary.PrintString` (`KismetStringLibrary.Concat_StrStr` "IsPunching: " (`KismetStringLibrary.Conv_BoolToString` (`self.IsPunching`))) true true (struct :`R` 1.0 :`G` 1.0 :`B` 1.0 :`A` 1.0) 0.0)
  (if (`self.NextPunch`)
    (`KismetSystemLibrary.PrintString` (`KismetStringLibrary.Concat_StrStr` "NextPunch: " "Left") true true (struct :`R` 1.0 :`G` 1.0 :`B` 1.0 :`A` 1.0) 0.0)
    (else
      (`KismetSystemLibrary.PrintString` (`KismetStringLibrary.Concat_StrStr` "NextPunch: " "Right") true true (struct :`R` 1.0 :`G` 1.0 :`B` 1.0 :`A` 1.0) 0.0))))

(event `self.L_Collision.OnComponentBeginOverlap`
  (params (OverlappedComponent :type "PrimitiveComponent Object Reference") (OtherActor :type "Actor Object Reference") (OtherComp :type "PrimitiveComponent Object Reference") (OtherBodyIndex :type Integer) (bFromSweep :type Boolean) (SweepResult :type "HitResult Structure (by ref)"))
  (bind _returnvalue (`self.GetComponentByClass` OtherActor "/Game/_Game/Blueprints/Components/BPA_Damageable.BPA_Damageable_C"))
  (if (`self.IsPunching`)
    (`/Engine/EditorBlueprintResources/StandardMacros.IsValid` _returnvalue
      (:`Is Valid`
        (`/Game/_Game/Blueprints/Components/BPA_Damageable.TakeDamage` _returnvalue 10)))))

(event `self.R_Collision.OnComponentBeginOverlap`
  (params (OverlappedComponent :type "PrimitiveComponent Object Reference") (OtherActor :type "Actor Object Reference") (OtherComp :type "PrimitiveComponent Object Reference") (OtherBodyIndex :type Integer) (bFromSweep :type Boolean) (SweepResult :type "HitResult Structure (by ref)"))
  (bind _returnvalue (`self.GetComponentByClass` OtherActor "/Game/_Game/Blueprints/Components/BPA_Damageable.BPA_Damageable_C"))
  (if (`self.IsPunching`)
    (`/Engine/EditorBlueprintResources/StandardMacros.IsValid` _returnvalue
      (:`Is Valid`
        (`/Game/_Game/Blueprints/Components/BPA_Damageable.TakeDamage` _returnvalue 10)))))

(fn `SetTargetR`
  (params (Position :type "Vector Structure")))

(fn `UserConstructionScript`)
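; BP_FollowCamera is a camera actor that becomes player 0's view target at BeginPlay and follows the group of BP_Character03 actors.
; Each Tick it interpolates toward their average position plus a scaled offset and sets the camera to a fixed angle.
; AveragedPositions searches for those characters on every call, printing their names and drawing a debug sphere at the midpoint.
; The construction script starts a looping EditorTick timer, but that function is empty.
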(event `self.ReceiveBeginPlay`
  (set `self.bFindCameraComponentWhenViewTarget` true)
  (`PlayerController.SetViewTargetWithBlend` (`GameplayStatics.GetPlayerController` 0) self 0.0 "VTBlend_Linear" 0.0 false))

(event `self.ReceiveTick`
  (params (DeltaSeconds :type "Float (single-precision)"))
  (bind _target (`self.AveragedPositions`))
  (`self.K2_SetActorLocation` (`KismetMathLibrary.VInterpTo` (`self.K2_GetActorLocation`) (+ _target (* (`self.Offset`) (`self.Length`))) (`GameplayStatics.GetWorldDeltaSeconds`) (`self.InterpSpeed`)))
  (`SceneComponent.K2_SetWorldRotation` (`self.Camera`) (`self.Angle`) false false))

(fn `AveragedPositions`
  (returns (Target :type "Vector Structure"))
  (locals (Sum :type "Vector Structure"))
  (bind _outactors (`GameplayStatics.GetAllActorsOfClass` "/Game/_Game/Blueprints/Actors/BP_Character03.BP_Character03_C"))
  (if (> (`KismetArrayLibrary.Array_Length` _outactors) 0)
    (for _array_element _outactors
      (`KismetSystemLibrary.PrintString` (`KismetSystemLibrary.GetDisplayName` _array_element) true true (struct :`G` 0.66 :`B` 1.0 :`A` 1.0) 0.0)
      (set `local.Sum` (+ (`self.K2_GetActorLocation` _array_element) (`local.Sum`))))
    (bind _returnvalue (/ (`local.Sum`) (`KismetArrayLibrary.Array_Length` _outactors)))
    (`KismetSystemLibrary.DrawDebugSphere` _returnvalue 20.0 12 (struct :`B` 1.0 :`A` 1.0) 0.0 2.0)
    (return _returnvalue)))

(fn `EditorTick`)

(fn `UserConstructionScript`
  (`KismetSystemLibrary.K2_SetTimer` null "EditorTick" 0.01 true))
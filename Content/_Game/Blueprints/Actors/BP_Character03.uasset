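; Player character with physics-driven movement, two-handed item combat and rope grabbing.
; Camera-relative input feeds capsule forces with manual drag and gravity over a traced ground plane, while mouse or stick steers facing separately.
; Facing dot products select nearby pickups for BPPickupAgent, which grabs or throws per hand with hold-to-charge meters.
; Held item type selects timeline-driven hand attacks or blocks; blocking slows movement, and falling below a height threshold triggers death.
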(event `self.ReceiveBeginPlay`
  ;[1 1 1] Inital setup
  (bind _returnvalue (`GameplayStatics.GetActorOfClass` "/Game/_Game/Blueprints/Actors/BP_FollowCamera.BP_FollowCamera_C"))
  (set `self.FollowCam` _returnvalue)
  (bind _output_get (set `self.Default_R` (`SceneComponent.GetRelativeTransform` (`self.Hand_R`))))
  (set `self.Default_R_Block` (`KismetMathLibrary.MakeTransform` (.location _output_get) (`KismetMathLibrary.MakeRotator` (.roll (.rotation _output_get)) 90.0 70.0) (.scale _output_get)))
  (bind _output_get_2 (set `self.Default_L` (`SceneComponent.GetRelativeTransform` (`self.Hand_L`))))
  (set `self.Default_L_Block` (`KismetMathLibrary.MakeTransform` (.location _output_get_2) (`KismetMathLibrary.MakeRotator` (.roll (.rotation _output_get_2)) 90.0 -70.0) (.scale _output_get_2)))
  (set `self.CanAttackRight` true)
  (set `CharacterMovementComponent.MaxWalkSpeed` (`self.MoveSpeed`) (`self.CharacterMovement`))
  (set `self.RotationDirection` (`KismetMathLibrary.Normal` (`self.GetActorForwardVector`)))
  (`/Game/_Game/Blueprints/Components/BPA_PickupAgent.SetHands` (`self.BP_PickupAgent`) (`self.Hand_R`) (`self.Hand_L`))
  (set `/Game/_Game/Blueprints/Components/BPA_Damageable.WidgetRef` (`WidgetComponent.GetUserWidgetObject` (`self.HealthBar`)) (`self.BPA_Damageable`)))

(event `InputAction|Jump`
  (params (Key :type "Key Structure"))
  (:`Pressed`
    (if (`self.IsGrounded`)
      (`PrimitiveComponent.AddImpulse` (`self.CapsuleComponent`) (0.0 0.0 50000.0) "None" false)
      (elif (`/Game/_Game/Blueprints/Components/BPA_RopeAgent.IsGrabbing` (`self.BPA_RopeAgent`))
        (`self.TryLaunchFromRope`)
        (`KismetSystemLibrary.PrintString` "Drop Rope")
        (else
          (`self.Try Grab Rope`)
          (`KismetSystemLibrary.PrintString` "Grab Rope"))))))

(event `InputAction|ThrowLeft`
  (params (Key :type "Key Structure"))
  (bind (_default_l_block_location _default_l_block_rotation) (`KismetMathLibrary.BreakTransform` (`self.Default_L_Block`)))
  (bind (_default_l_location _default_l_rotation) (`KismetMathLibrary.BreakTransform` (`self.Default_L`)))
  ;[1 1 1] Throw/Pickup Left
  (:`Pressed`
    (`/Engine/EditorBlueprintResources/StandardMacros.IsValid` (`/Game/_Game/Blueprints/Components/BPA_PickupAgent.ObjectLeft` (`self.BP_PickupAgent`))
      (:`Is Valid`
        (set `self.ThrowLeftPressed` true))
      (:`Is Not Valid`
        (`/Game/_Game/Blueprints/Components/BPA_PickupAgent.PickupLeft` (`self.BP_PickupAgent`))
        (set `/Game/_Game/Blueprints/Components/BPA_PickupAgent.LeftGrabbedFrame` true (`self.BP_PickupAgent`))
        (bind _objectleft (`/Game/_Game/Blueprints/Components/BPA_PickupAgent.ObjectLeft` (`self.BP_PickupAgent`))
          (:`then`
            (if (`|EnumEquality` (`/Game/_Game/Blueprints/Components/BPA_Pickup.Type` _objectleft) "NewEnumerator0")
              (`SceneComponent.K2_SetRelativeRotation` (`self.Hand_L`) _default_l_block_rotation false false)))
          (:`else`)))))
  (:`Released`
    (if (`/Game/_Game/Blueprints/Components/BPA_PickupAgent.LeftGrabbedFrame` (`self.BP_PickupAgent`))
      (set `/Game/_Game/Blueprints/Components/BPA_PickupAgent.LeftGrabbedFrame` false (`self.BP_PickupAgent`))
      (else
        (set `self.ThrowLeftPressed` false)
        (`/Game/_Game/Blueprints/Components/BPA_PickupAgent.DropLeft` (`self.BP_PickupAgent`) (* (`self.RotationDirection`) (`self.ThrowMeterL`)))
        (`SceneComponent.K2_SetRelativeRotation` (`self.Hand_L`) _default_l_rotation false false)))))

(event `InputAction|ThrowRight`
  (params (Key :type "Key Structure"))
  (bind (_default_r_location _default_r_rotation) (`KismetMathLibrary.BreakTransform` (`self.Default_R`)))
  (bind (_default_r_block_location _default_r_block_rotation) (`KismetMathLibrary.BreakTransform` (`self.Default_R_Block`)))
  ;[1 1 1] Throw/Pickup Right
  (:`Pressed`
    (`/Engine/EditorBlueprintResources/StandardMacros.IsValid` (`/Game/_Game/Blueprints/Components/BPA_PickupAgent.ObjectRight` (`self.BP_PickupAgent`))
      (:`Is Valid`
        (set `self.ThrowRightPressed` true))
      (:`Is Not Valid`
        (`/Game/_Game/Blueprints/Components/BPA_PickupAgent.PickupRight` (`self.BP_PickupAgent`))
        (set `/Game/_Game/Blueprints/Components/BPA_PickupAgent.RightGrabbedFrame` true (`self.BP_PickupAgent`))
        (bind _objectright (`/Game/_Game/Blueprints/Components/BPA_PickupAgent.ObjectRight` (`self.BP_PickupAgent`))
          (:`then`
            (if (`|EnumEquality` (`/Game/_Game/Blueprints/Components/BPA_Pickup.Type` _objectright) "NewEnumerator0")
              (`SceneComponent.K2_SetRelativeRotation` (`self.Hand_R`) _default_r_block_rotation false false)))
          (:`else`)))))
  (:`Released`
    (if (`/Game/_Game/Blueprints/Components/BPA_PickupAgent.RightGrabbedFrame` (`self.BP_PickupAgent`))
      (set `/Game/_Game/Blueprints/Components/BPA_PickupAgent.RightGrabbedFrame` false (`self.BP_PickupAgent`))
      (else
        (set `self.ThrowRightPressed` false)
        (`/Game/_Game/Blueprints/Components/BPA_PickupAgent.DropRight` (`self.BP_PickupAgent`) (* (`self.RotationDirection`) (`self.ThrowMeterR`)))
        (`SceneComponent.K2_SetRelativeRotation` (`self.Hand_R`) _default_r_rotation false false)))))

(event `InputAxis|Move Right / Left`
  (params (AxisValue :type "Float (single-precision)"))
  ;[1 1 1] Locomotion
  (set `self.MoveRightVec` (* AxisValue (`self.GetActorRightVector` (`self.FollowCam`)))))

(event `InputAxis|Move Forward / Backward`
  (params (AxisValue :type "Float (single-precision)"))
  ;[1 1 1] Locomotion
  (set `self.MoveLeftVec` (* AxisValue (`self.GetActorForwardVector` (`self.FollowCam`)))))

(event `InputAxis|Turn Right / Left Mouse`
  (params (AxisValue :type "Float (single-precision)"))
  ;[1 1 1] Locomotion
  (set `self.RotationDirection` (`KismetMathLibrary.RotateAngleAxis` (`self.RotationDirection`) (* AxisValue (`self.RotationSpeed`)) (0.0 0.0 1.0))))

(event `InputAxis|Turn Right / Left Gamepad`
  (params (AxisValue :type "Float (single-precision)"))
  ;[1 1 1] Locomotion
  ;;[1 1 1] Gamepad rotation
  (set `self.RightDir` (* AxisValue (`self.GetActorRightVector` (`self.FollowCam`)))))

(event `InputAxis|Look Up / Down Gamepad`
  (params (AxisValue :type "Float (single-precision)"))
  ;[1 1 1] Locomotion
  ;;[1 1 1] Gamepad rotation
  (set `self.LeftDir` (* AxisValue (`self.GetActorForwardVector` (`self.FollowCam`)) -1.0)))

(event `InputAction|AttackRight`
  (params (Key :type "Key Structure"))
  ;[1 1 1] Combat
  (:`Pressed`
    (bind _objectright (`/Game/_Game/Blueprints/Components/BPA_PickupAgent.ObjectRight` (`self.BP_PickupAgent`))
      (:`then`
        (if (`|EnumEquality` (`/Game/_Game/Blueprints/Components/BPA_Pickup.Type` _objectright) "NewEnumerator1")
          (if (or (`self.IsBlockingRight`) (`self.IsBlockingLeft`))
            _
            (elif (`self.CanAttackRight`)
              (set `self.IsAttackingRight` true)
              (set `self.CanAttackRight` false)
              (set `/Game/_Game/Blueprints/Components/BPA_Pickup.IsAttacking` true (`/Game/_Game/Blueprints/Components/BPA_PickupAgent.ObjectRight` (`self.BP_PickupAgent`)))
              (set `self.DotToAdd` (`self.MovRotDot`))
              (bind (_direction _translation _rotation) (`Timeline|AttackR_Timeline` :!via `PlayFromStart`)
                (:`Update`
                  (bind (_x _y _z) (`KismetMathLibrary.BreakVector3f` _rotation))
                  (`self.AddLocRotRightHand` _translation (`KismetMathLibrary.MakeVector` (* (`self.DotToAdd`) _x) _y _z) (`self.Default_R`)))
                (:`Finished`
                  (set `self.CanAttackRight` true)
                  (set `self.IsAttackingRight` false)
                  (bind _objectright_2 (`/Game/_Game/Blueprints/Components/BPA_PickupAgent.ObjectRight` (`self.BP_PickupAgent`))
                    (:`then`
                      (set `/Game/_Game/Blueprints/Components/BPA_Pickup.IsAttacking` false _objectright_2))
                    (:`else`))))))
          (else
            (set `self.IsBlockingRight` true)
            (bind (_direction_2 _translation_2 _rotation_2) (`Timeline|BlockR_Timeline` :!label _label)
              (:`Update`
                (`self.AddLocRotRightHand` _translation_2 _rotation_2 (`self.Default_R_Block`)))))))
      (:`else`)))
  (:`Released`
    (bind _objectright_3 (`/Game/_Game/Blueprints/Components/BPA_PickupAgent.ObjectRight` (`self.BP_PickupAgent`))
      (:`then`
        (if (`|EnumEquality` (`/Game/_Game/Blueprints/Components/BPA_Pickup.Type` _objectright_3) "NewEnumerator0")
          (set `self.IsBlockingRight` false)
          (goto _label :!via `Reverse`)))
      (:`else`))))

(event `InputAction|AttackLeft`
  (params (Key :type "Key Structure"))
  ;[1 1 1] Combat
  (:`Pressed`
    (bind _objectleft (`/Game/_Game/Blueprints/Components/BPA_PickupAgent.ObjectLeft` (`self.BP_PickupAgent`))
      (:`then`
        (if (`|EnumEquality` (`/Game/_Game/Blueprints/Components/BPA_Pickup.Type` _objectleft) "NewEnumerator1")
          (if (or (`self.IsBlockingRight`) (`self.IsBlockingLeft`))
            _
            (elif (`self.CanAttackLeft`)
              (set `self.IsAttackingLeft` true)
              (set `self.CanAttackLeft` false)
              (set `/Game/_Game/Blueprints/Components/BPA_Pickup.IsAttacking` true (`/Game/_Game/Blueprints/Components/BPA_PickupAgent.ObjectLeft` (`self.BP_PickupAgent`)))
              (set `self.DotToAdd` (`self.MovRotDot`))
              (bind (_direction _translation _rotation) (`Timeline|AttackL_Timeline` :!via `PlayFromStart`)
                (:`Update`
                  (bind (_x _y _z) (`KismetMathLibrary.BreakVector3f` _rotation))
                  (`self.AddLockRotLeftHand` _translation (`KismetMathLibrary.MakeVector` (* (`self.DotToAdd`) _x) _y _z) (`self.Default_L`)))
                (:`Finished`
                  (set `self.CanAttackLeft` true)
                  (set `self.IsAttackingLeft` false)
                  (set `/Game/_Game/Blueprints/Components/BPA_Pickup.IsAttacking` false (`/Game/_Game/Blueprints/Components/BPA_PickupAgent.ObjectLeft` (`self.BP_PickupAgent`)))))))
          (else
            (set `self.IsBlockingLeft` true)
            (bind (_direction_2 _translation_2 _rotation_2) (`Timeline|BlockL_Timeline` :!label _label_2)
              (:`Update`
                (`self.AddLockRotLeftHand` _translation_2 _rotation_2 (`self.Default_L_Block`)))))))
      (:`else`)))
  (:`Released`
    (bind _objectleft_2 (`/Game/_Game/Blueprints/Components/BPA_PickupAgent.ObjectLeft` (`self.BP_PickupAgent`))
      (:`then`
        (if (`|EnumEquality` (`/Game/_Game/Blueprints/Components/BPA_Pickup.Type` _objectleft_2) "NewEnumerator0")
          (set `self.IsBlockingLeft` false)
          (goto _label_2 :!via `Reverse`)))
      (:`else`))))

(event `self.ReceiveTick`
  (params (DeltaSeconds :type "Float (single-precision)"))
  (bind _returnvalue (`self.K2_GetActorLocation`))
  (bind (_returnvalue_x _returnvalue_y _returnvalue_z) (`KismetMathLibrary.BreakVector` (`self.K2_GetActorLocation`)))
  (bind _returnvalue_2 (`self.K2_GetActorLocation`))
  (bind _returnvalue_3 (`self.K2_GetActorLocation`))
  (bind _returnvalue_4 (`self.K2_GetActorLocation`))
  (bind _returnvalue_5 (`self.K2_GetActorLocation`))
  (bind (_returnvalue_roll _returnvalue_pitch _returnvalue_yaw) (`KismetMathLibrary.BreakRotator` (`KismetMathLibrary.RInterpTo` (`self.CurrentRotation`) (`KismetMathLibrary.FindLookAtRotation` (`KismetMathLibrary.Vector_Zero`) (`self.RotationDirection`)) (`GameplayStatics.GetWorldDeltaSeconds`) 5.0)))
  (bind (_returnvalue_x_2 _returnvalue_y_2) (`KismetMathLibrary.BreakVector` (+ _returnvalue_3 (* (`KismetMathLibrary.Normal` (`self.RotationDirection`)) 100.0))))
  (`|ExecutionSequence`
    (:`then_0`
      (if (`self.Debug`)
        (`KismetSystemLibrary.DrawDebugLine` _returnvalue_3 (`KismetMathLibrary.MakeVector` _returnvalue_x_2 _returnvalue_y_2 (`.Z` (`KismetMathLibrary.BreakVector3f` _returnvalue_3))) (struct :`R` 1.0 :`A` 1.0) 0.0 4.0)
        (`/Game/_Game/Blueprints/BP_UtilityLib.LogBool` "IsBlockingRight" (`self.IsBlockingRight`))
        (`/Game/_Game/Blueprints/BP_UtilityLib.LogBool` "IsBlockingLeft" (`self.IsBlockingLeft`))
        (`/Game/_Game/Blueprints/BP_UtilityLib.LogBool` "CanAttack" (`self.CanAttackRight`))
        (`/Game/_Game/Blueprints/BP_UtilityLib.LogVec` "MovementInput" (`self.MovementInput`))
        (`/Game/_Game/Blueprints/BP_UtilityLib.LogVec` "RotationDirection" (`self.RotationDirection`))
        (`KismetSystemLibrary.DrawDebugLine` _returnvalue_5 (+ _returnvalue_5 (* (`KismetMathLibrary.Normal` (`self.MovementInput`)) 75.0)) (struct :`B` 1.0 :`A` 1.0) 0.0 4.0)
        (`KismetSystemLibrary.DrawDebugLine` (+ _returnvalue_4 (0.0 0.0 2.0)) (+ (+ _returnvalue_4 (* (`self.RotationDirection`) (`self.ThrowMeterR`) 100.0)) (0.0 0.0 2.0)) (struct :`G` 0.870588 :`B` 1.0 :`A` 1.0) 0.0 6.0)
        (`/Game/_Game/Blueprints/BP_UtilityLib.LogString` "SelectedPickup" (`KismetSystemLibrary.GetDisplayName` (`/Game/_Game/Blueprints/Components/BPA_PickupAgent.SelectedPickup` (`self.BP_PickupAgent`))))
        (`KismetSystemLibrary.DrawDebugLine` (+ _returnvalue_2 (0.0 0.0 2.0)) (+ (+ _returnvalue_2 (* (`self.RotationDirection`) (`self.ThrowMeterL`) 100.0)) (0.0 0.0 2.0)) (struct :`G` 0.870588 :`B` 1.0 :`A` 1.0) 0.0 6.0)))
    (:`then_1`
      (if (or (`self.IsBlockingRight`) (`self.IsBlockingLeft`))
        (set `CharacterMovementComponent.MaxWalkSpeed` (* (`self.MoveSpeed`) 0.5) (`self.CharacterMovement`))
        (else
          (set `CharacterMovementComponent.MaxWalkSpeed` (`self.MoveSpeed`) (`self.CharacterMovement`)))))
    (:`then_2`
      ;[1 1 1] Character Rotation
      (set `self.MovementInput` (+ (`self.MoveRightVec`) (`self.MoveLeftVec`)))
      (bind _output_get (set `self.RotationInput` (+ (`self.LeftDir`) (`self.RightDir`))))
      (if (> (`KismetMathLibrary.VSize` _output_get) 0.0)
        (set `self.RotationDirection` (`self.RotationInput`)))
      (bind _output_get_2 (set `self.CurrentRotation` (`KismetMathLibrary.MakeRotator` 0.0 0.0 _returnvalue_yaw)))
      (`self.K2_SetActorRotation` (`KismetMathLibrary.MakeRotator` 0.0 0.0 (.yaw _output_get_2))))
    (:`then_3`
      (`self.ClosestPickup`)
      (`self.RightMeter`)
      (`self.LeftMeter`))
    (:`then_4`
      ;[1 1 1] Locomotion
      (if (`self.IsGrounded`)
        (if (or (`self.IsBlockingRight`) (`self.IsBlockingLeft`))
          (set `self.CurrentSpeed` 80000.0)
          (else
            (set `self.CurrentSpeed` 120000.0)))
        (elif (`/Game/_Game/Blueprints/Components/BPA_RopeAgent.IsGrabbing` (`self.BPA_RopeAgent`))
          (set `self.CurrentSpeed` 10000.0)
          (else
            (set `self.CurrentSpeed` 10000.0))))
      (`PrimitiveComponent.AddForce` (`self.CapsuleComponent`) (* (`KismetMathLibrary.ProjectVectorOnToPlane` (`KismetMathLibrary.Normal` (+ (`self.MoveRightVec`) (`self.MoveLeftVec`))) (`self.GroundNormal`)) (`self.CurrentSpeed`)) "None" false)
      (`PrimitiveComponent.AddForce` (`self.CapsuleComponent`) (* (`KismetMathLibrary.NegateVector` (`SceneComponent.GetComponentVelocity` (`self.CapsuleComponent`))) 100.0) "None" false)
      (if (`/Game/_Game/Blueprints/Components/BPA_RopeAgent.IsGrabbing` (`self.BPA_RopeAgent`))
        (`PrimitiveComponent.AddForce` (`self.CapsuleComponent`) (0.0 0.0 0.0) "None" false)
        (`KismetSystemLibrary.PrintString` "Zero Gravity" true true (struct :`G` 0.66 :`B` 1.0 :`A` 1.0) 0.0)
        (elif (`self.IsGrounded`)
          (`PrimitiveComponent.AddForce` (`self.CapsuleComponent`) (0.0 0.0 -100000.0) "None" false)
          (else
            (`PrimitiveComponent.AddForce` (`self.CapsuleComponent`) (0.0 0.0 -150000.0) "None" false)))))
    (:`then_5`
      (`self.WidgetLookAtCamera`)
      (set `self.MovRotDot` (`KismetMathLibrary.Dot_VectorVector` (`self.MovementInput`) (`KismetMathLibrary.RotateAngleAxis` (`self.RotationDirection`) 90.0 (0.0 0.0 1.0)))))
    (:`then_6`
      (bind (_outhit _returnvalue_6) (`KismetSystemLibrary.LineTraceSingleForObjects` _returnvalue (+ _returnvalue (* (`KismetMathLibrary.Vector_Down`) 75.0)) (`|MakeArray` "ObjectTypeQuery9" :!type "EObjectTypeQuery Enum") false (`|MakeArray` self :!type "Actor Object Reference") "ForOneFrame" true (struct :`R` 1.0 :`A` 1.0) (struct :`G` 1.0 :`A` 1.0) 0.0))
      (set `self.IsGrounded` _returnvalue_6)
      (bind (_bblockinghit _binitialoverlap _time _distance _location _impactpoint _normal) (`GameplayStatics.BreakHitResult` _outhit))
      (bind _output_get_3 (set `self.GroundNormal` _normal))
      (`KismetSystemLibrary.DrawDebugLine` _location (+ (* _output_get_3 100.0) _location) (struct :`B` 1.0 :`A` 1.0) 0.0 2.0))
    (:`then_7`
      (if (<= _returnvalue_z -10.0)
        (`/Game/_Game/Blueprints/Components/BPA_Damageable.OnDeath` (`self.BPA_Damageable`))))))

(event `self.PickupRange.OnComponentBeginOverlap`
  (params (OverlappedComponent :type "PrimitiveComponent Object Reference") (OtherActor :type "Actor Object Reference") (OtherComp :type "PrimitiveComponent Object Reference") (OtherBodyIndex :type Integer) (bFromSweep :type Boolean) (SweepResult :type "HitResult Structure (by ref)"))
  (bind _returnvalue (`self.GetComponentByClass` OtherActor "/Game/_Game/Blueprints/Components/BPA_Pickup.BPA_Pickup_C"))
  ;[1 1 1] Pickup range
  (`/Engine/EditorBlueprintResources/StandardMacros.IsValid` _returnvalue
    (:`Is Valid`
      (`KismetArrayLibrary.Array_AddUnique` (`self.PickupsInRange`) _returnvalue))))

(event `self.PickupRange.OnComponentEndOverlap`
  (params (OverlappedComponent :type "PrimitiveComponent Object Reference") (OtherActor :type "Actor Object Reference") (OtherComp :type "PrimitiveComponent Object Reference") (OtherBodyIndex :type Integer))
  (bind _returnvalue (`self.GetComponentByClass` OtherActor "/Game/_Game/Blueprints/Components/BPA_Pickup.BPA_Pickup_C"))
  ;[1 1 1] Pickup range
  (`/Engine/EditorBlueprintResources/StandardMacros.IsValid` _returnvalue
    (:`Is Valid`
      (if (`KismetArrayLibrary.Array_Contains` (`self.PickupsInRange`) _returnvalue)
        (`KismetArrayLibrary.Array_RemoveItem` (`self.PickupsInRange`) _returnvalue)
        (set `/Game/_Game/Blueprints/Components/BPA_Pickup.IsSelected` false _returnvalue)
        (set `/Game/_Game/Blueprints/Components/BPA_PickupAgent.SelectedPickup` null (`self.BP_PickupAgent`))))))

(fn `AddLockRotLeftHand`
  (params (Offset :type "Vector Structure") (Rotation :type "Vector3f Structure") (Default :type "Transform Structure (by ref)"))
  (bind (_x _y _z) (`KismetMathLibrary.BreakVector3f` Rotation))
  (`SceneComponent.K2_SetRelativeLocationAndRotation` (`self.Hand_L`) (+ Offset (.location Default)) (`KismetMathLibrary.ComposeRotators` (`KismetMathLibrary.MakeRotator` _x _y _z) (.rotation Default)) false false))

(fn `AddLocRotRightHand`
  (params (Offset :type "Vector Structure") (Rotation :type "Vector3f Structure") (Default :type "Transform Structure (by ref)"))
  (bind (_x _y _z) (`KismetMathLibrary.BreakVector3f` Rotation))
  (`SceneComponent.K2_SetRelativeLocationAndRotation` (`self.Hand_R`) (+ Offset (.location Default)) (`KismetMathLibrary.ComposeRotators` (`KismetMathLibrary.MakeRotator` _x _y _z) (.rotation Default)) false false))

(fn `ClosestPickup`
  (locals (MaxDot :type "Float (double-precision)") (CurrentDot :type "Float (double-precision)" :default 0.0) (MinDotIndex :type Integer) (CurrentIndex :type Integer) (MinPickup :type "/Game/_Game/Blueprints/Components/BPA_Pickup Object Reference") (CurrentPickup :type "/Game/_Game/Blueprints/Components/BPA_Pickup Object Reference"))
  (bind _returnvalue (`self.K2_GetActorLocation`))
  (bind _minpickup (`local.MinPickup`))
  (if (> (`KismetArrayLibrary.Array_Length` (`self.PickupsInRange`)) 0)
    (set `local.CurrentIndex` -1)
    (set `local.MaxDot` 0.0)
    (for _array_element (`self.PickupsInRange`)
      (bind _output_get (set `local.CurrentPickup` _array_element))
      (set `/Game/_Game/Blueprints/Components/BPA_Pickup.IsSelected` false _output_get)
      (bind _returnvalue_2 (`SceneComponent.K2_GetComponentLocation` (`/Game/_Game/Blueprints/Components/BPA_Pickup.Center` _array_element)))
      (bind (_x _y) (`KismetMathLibrary.BreakVector3f` _returnvalue_2))
      (bind _returnvalue_3 (`KismetMathLibrary.MakeVector` _x _y (`.Z` (`KismetMathLibrary.BreakVector3f` _returnvalue))))
      (`KismetSystemLibrary.DrawDebugLine` _returnvalue _returnvalue_3 (struct :`R` 1.0 :`B` 0.029831 :`A` 1.0) 0.0 3.0)
      (`KismetSystemLibrary.DrawDebugLine` _returnvalue_2 _returnvalue_3 (struct :`R` 1.0 :`A` 1.0) 0.0 3.0)
      (bind _output_get_2 (set `local.CurrentDot` (`KismetMathLibrary.Dot_VectorVector` (`KismetMathLibrary.Normal` (- _returnvalue_3 _returnvalue)) (`KismetMathLibrary.Normal` (`self.RotationDirection`)))))
      (if (>= _output_get_2 0.6)
        (if (> (`local.CurrentDot`) (`local.MaxDot`))
          (set `local.MinPickup` (`local.CurrentPickup`)))))
    (`/Engine/EditorBlueprintResources/StandardMacros.IsValid` (`local.MinPickup`)
      (:`Is Valid`
        (`KismetSystemLibrary.DrawDebugLine` (`self.K2_GetActorLocation`) (`SceneComponent.K2_GetComponentLocation` (`/Game/_Game/Blueprints/Components/BPA_Pickup.Center` (`local.MinPickup`))) (struct :`G` 1.0 :`B` 0.068 :`A` 1.0) 0.0 4.0)
        (set `/Game/_Game/Blueprints/Components/BPA_PickupAgent.SelectedPickup` _minpickup (`self.BP_PickupAgent`))
        (set `/Game/_Game/Blueprints/Components/BPA_Pickup.IsSelected` true _minpickup))
      (:`Is Not Valid`
        (set `/Game/_Game/Blueprints/Components/BPA_PickupAgent.SelectedPickup` null (`self.BP_PickupAgent`))))
    (else
      (return))))

(fn `LeftMeter`
  (if (`self.ThrowLeftPressed`)
    (bind _output_get (set `self.ThrowMeterL` (`KismetMathLibrary.FClamp` (+ (`self.ThrowMeterL`) (`GameplayStatics.GetWorldDeltaSeconds`)))))
    (`/Game/_Game/Blueprints/BP_UtilityLib.LogFloat` "ThrowL" _output_get)
    (else
      (bind _output_get_2 (set `self.ThrowMeterL` 0.0))
      (`/Game/_Game/Blueprints/BP_UtilityLib.LogFloat` "ThrowL" _output_get_2))))

(fn `OnHit`)

(fn `RightMeter`
  (if (`self.ThrowRightPressed`)
    (set `self.ThrowMeterR` (`KismetMathLibrary.FClamp` (+ (`self.ThrowMeterR`) (`GameplayStatics.GetWorldDeltaSeconds`))))
    (else
      (set `self.ThrowMeterR` 0.0))))

(fn `SetTargetR`
  (params (Position :type "Vector Structure")))

(fn `Try Grab Rope`
  (bind _capsulecomponent (`self.CapsuleComponent`))
  (bind _overlappingactors (`PrimitiveComponent.GetOverlappingActors` (`self.CapsuleComponent`) "/Script/Brawler_Prototype.GrabbableRope"))
  (bind (_distance _returnvalue) (`GameplayStatics.FindNearestActor` (`self.K2_GetActorLocation`) _overlappingactors))
  (`KismetArrayLibrary.Array_Add` _overlappingactors (`self.ClosestRope`))
  (`KismetSystemLibrary.PrintString` (`KismetStringLibrary.Conv_IntToString` (`KismetArrayLibrary.Array_Length` _overlappingactors)))
  (`/Engine/EditorBlueprintResources/StandardMacros.IsValid` _returnvalue
    (:`Is Valid`
      (bind _asgrabbable_rope (cast `GrabbableRope` _returnvalue))
      (bind _output_get (set `self.closestRope` _asgrabbable_rope))
      (`GrabbableRope.AttachPlayer` _output_get self (`self.CapsuleComponent`))
      (`PrimitiveComponent.SetSimulatePhysics` _capsulecomponent true)
      (`PrimitiveComponent.WakeAllRigidBodies` _capsulecomponent)
      (`PrimitiveComponent.SetConstraintMode` (`self.CapsuleComponent`) "None"))))

(fn `TryLaunchFromRope`
  (bind _closestrope (`self.ClosestRope`))
  (`/Engine/EditorBlueprintResources/StandardMacros.IsValid` _closestrope
    (:`Is Valid`
      (`self.K2_SetActorRotation` (struct))
      (`GrabbableRope.DetachPlayer` _closestrope)
      (`self.LaunchCharacter` (`self.GetVelocity`) true true)
      (set `self.closestRope` null) ; clear the stored rope
      (`PrimitiveComponent.SetConstraintMode` (`self.CapsuleComponent`) "Default"))))

(fn `UserConstructionScript`)

(fn `WidgetLookAtCamera`
  (bind _followcam (`self.FollowCam`)
    (:`then`
      (`SceneComponent.K2_SetWorldRotation` (`self.HealthBar`) (`KismetMathLibrary.FindLookAtRotation` (`self.K2_GetActorLocation`) (`self.K2_GetActorLocation` _followcam)) false false))
    (:`else`)))
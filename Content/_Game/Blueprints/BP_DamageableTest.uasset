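; BP_DamageableTest is a test actor for the BPADamageable component, with a world-space widget that faces the follow camera.
; On BeginPlay it hands the widget's user object to BPADamageable and caches the BP_FollowCamera found in the level.
; Each Tick it rotates the widget toward that camera and destroys the actor once the component's Health drops to zero or below.
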(event `self.ReceiveBeginPlay`
  (set `/Game/_Game/Blueprints/BPA_Damageable.WidgetRef` (`WidgetComponent.GetUserWidgetObject` (`self.Widget`)) (`self.BPA_Damageable`))
  (bind _returnvalue (`GameplayStatics.GetActorOfClass` "/Game/_Game/Blueprints/BP_FollowCamera.BP_FollowCamera_C"))
  (set `self.CameraRef` _returnvalue))

(event `self.ReceiveTick`
  (params (DeltaSeconds :type "Float (single-precision)"))
  (`SceneComponent.K2_SetWorldRotation` (`self.Widget`) (`KismetMathLibrary.FindLookAtRotation` (`self.K2_GetActorLocation`) (`self.K2_GetActorLocation` (`self.CameraRef`))) false false)
  (if (<= (`/Game/_Game/Blueprints/BPA_Damageable.Health` (`self.BPA_Damageable`)) 0)
    (`self.K2_DestroyActor`)))

(fn `UserConstructionScript`)
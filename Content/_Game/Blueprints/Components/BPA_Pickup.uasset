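; Pickup component that lets an agent hold, drop or throw its owning actor and hit targets with it.
; While held, physics is off and Tick sweeps the root to the hand's transform instead of attaching; dropping restores physics and applies an impulse.
; When free, selection tints the material by Block or Attack type.
; Hits damage and knock back targets; depleted condition destroys the item, though hits currently subtract zero condition.
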(event `self.ReceiveTick`
  (params (DeltaSeconds :type "Float (single-precision)"))
  (bind _rootcomponent (`Actor.RootComponent` (`self.GetOwner`)))
  (bind (_returnvalue_location _returnvalue_rotation _returnvalue_scale) (`KismetMathLibrary.BreakTransform` (`SceneComponent.K2_GetComponentToWorld` _rootcomponent)))
  (if (not (`self.Held`))
    (if (`self.IsSelected`)
      (`self.HoverIn`)
      (else
        (`self.HoverOut`)))
    (else
      (`/Engine/EditorBlueprintResources/StandardMacros.IsValid` (`self.AttachedHand`)
        (:`Is Valid`
          (`SceneComponent.K2_SetWorldTransform` _rootcomponent (`KismetMathLibrary.MakeTransform` (.location (`SceneComponent.K2_GetComponentToWorld` (`self.AttachedHand`))) (.rotation (`SceneComponent.K2_GetComponentToWorld` (`self.AttachedHand`))) _returnvalue_scale) true false))))))

(fn `AttachTick`)

(fn `HoverIn`
  (switch `/Game/_Game/Blueprints/Enum_PickupType` (`self.Type`)
    (:`NewEnumerator0`
      (`MaterialInstanceDynamic.SetVectorParameterValue` (`self.Material`) "Color" (struct :`R` 0.145833 :`G` 0.145833 :`B` 1.0 :`A` 1.0)))
    (:`NewEnumerator1`
      (`MaterialInstanceDynamic.SetVectorParameterValue` (`self.Material`) "Color" (struct :`R` 1.0 :`G` 0.098958 :`B` 0.122853 :`A` 1.0)))))

(fn `HoverOut`
  (`MaterialInstanceDynamic.SetVectorParameterValue` (`self.Material`) "Color" (struct :`R` 0.545098 :`G` 0.545098 :`B` 0.545098 :`A` 1.0)))

(fn `IsHeld`
  (returns (Held :type Boolean))
  (return (`self.Held`)))

(fn `LoseCondition`
  (params (Damage :type Integer))
  (bind _output_get (set `self.Condition` (- (`self.Condition`) Damage)))
  (if (<= _output_get 0)
    (`self.OnDestroy`)))

(fn `OnDestroy`
  (bind _returnvalue (`self.GetOwner`))
  (`self.OnDrop` (0.0 0.0 0.0))
  (`Actor.K2_DestroyActor` _returnvalue)
  (`/Game/_Game/Blueprints/BP_UtilityLib.LogString` "Destroyed" (`KismetSystemLibrary.GetDisplayName` _returnvalue) 1.0 (struct :`R` 1.0 :`A` 1.0)))

(fn `OnDrop`
  (params (ForceVec :type "Vector Structure"))
  (locals (RootRef :type "StaticMeshComponent Object Reference") (ForceRef :type "Vector Structure"))
  (set `local.ForceRef` ForceVec)
  (bind _asstatic_mesh_component (cast `StaticMeshComponent` (`Actor.RootComponent` (`self.GetOwner`))))
  (bind _output_get (set `local.RootRef` _asstatic_mesh_component))
  (`PrimitiveComponent.SetSimulatePhysics` _output_get true)
  (`PrimitiveComponent.SetCollisionEnabled` (`local.RootRef`) "QueryAndPhysics")
  (`Actor.K2_DetachFromActor` (`self.GetOwner`) "KeepWorld" "KeepWorld" "KeepWorld")
  (`PrimitiveComponent.AddImpulse` (`local.RootRef`) (`local.ForceRef`) "None" false)
  (set `self.Held` false)
  (set `self.AttachedHand` null)
  (set `self.HeldByAgent` null))

(fn `OnGetHit`)

(fn `OnHit`
  (params (DamageRef :type "/Game/_Game/Blueprints/Components/BPA_Damageable Object Reference") (Hit :type "HitResult Structure (by ref)"))
  (locals (LocalDamageRef :type "/Game/_Game/Blueprints/Components/BPA_Damageable Object Reference"))
  (bind (_returnvalue_x _returnvalue_y) (`KismetMathLibrary.BreakVector` (- (`Actor.K2_GetActorLocation` (`self.GetOwner` (`local.LocalDamageRef`))) (`.Location` (`GameplayStatics.BreakHitResult` Hit)))))
  (`/Engine/EditorBlueprintResources/StandardMacros.IsValid` DamageRef
    (:`Is Valid`
      (bind _output_get (set `local.LocalDamageRef` DamageRef))
      (`/Game/_Game/Blueprints/Components/BPA_Damageable.OnHit` _output_get (`self.Damage`))
      (`self.LoseCondition` 0)
      (bind _asprimitive_component (cast `PrimitiveComponent` (`Actor.RootComponent` (`self.GetOwner` (`local.LocalDamageRef`)))))
      (`PrimitiveComponent.AddImpulse` _asprimitive_component (* (`KismetMathLibrary.Normal` (`KismetMathLibrary.MakeVector` _returnvalue_x _returnvalue_y)) 50000.0) "None" false))))

(fn `OnPickup`
  (params (HandComponent :type "StaticMeshComponent Object Reference") (Agent :type "/Game/_Game/Blueprints/Components/BPA_PickupAgent Object Reference"))
  (locals (RootRef :type "StaticMeshComponent Object Reference") (HandRef :type "StaticMeshComponent Object Reference"))
  (bind _asstatic_mesh_component (cast `StaticMeshComponent` (`Actor.RootComponent` (`self.GetOwner`))))
  (set `local.HandRef` HandComponent)
  (bind _output_get (set `local.RootRef` _asstatic_mesh_component))
  (`PrimitiveComponent.SetSimulatePhysics` _output_get false)
  (set `self.HeldByAgent` Agent)
  (`PrimitiveComponent.SetCollisionEnabled` (`local.RootRef`) "QueryOnly")
  (set `self.AttachedHand` (`local.HandRef`))
  (set `self.Held` true)
  (`self.HoverOut`))

(fn `SetHoldLocation`
  (params (HoldLocation :type "SceneComponent Object Reference"))
  (set `self.HoldLocation` HoldLocation))

(fn `SetMaterialInstance`
  (params (MatInstance :type "MaterialInstanceDynamic Object Reference"))
  (set `self.Material` MatInstance))
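; Actor component that lets its owner pick up, hold and throw pickup objects with a left and a right hand.
; SetHands stores the two hand components, and each pickup function hands a valid, unheld SelectedPickup to that hand via OnPickup, then clears the selection.
; Each drop function passes a direction scaled by ThrowStrength to OnDrop, clears the held object and selection, and logs a debug message.
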(fn `DropLeft`
  (params (Direction :type "Vector Structure"))
  (bind _objectleft (`self.ObjectLeft`)
    (:`then`
      (`/Game/_Game/Blueprints/Components/BPA_Pickup.OnDrop` _objectleft (* Direction (`self.ThrowStrength`)))
      ;[1 1 1] Debug
      (`/Game/_Game/Blueprints/BP_UtilityLib.LogString` "Dropped" (`KismetSystemLibrary.GetDisplayName` (`self.GetOwner`)) 1.0 (struct :`R` 1.0 :`A` 1.0))
      (set `self.ObjectLeft` null)
      (set `self.SelectedPickup` null))
    (:`else`)))

(fn `DropRight`
  (params (Direction :type "Vector Structure"))
  (bind _objectright (`self.ObjectRight`)
    (:`then`
      (`/Game/_Game/Blueprints/Components/BPA_Pickup.OnDrop` _objectright (* Direction (`self.ThrowStrength`)))
      ;[1 1 1] Debug
      (`/Game/_Game/Blueprints/BP_UtilityLib.LogString` "Dropped" (`KismetSystemLibrary.GetDisplayName` (`self.GetOwner` _objectright)) 1.0 (struct :`R` 1.0 :`A` 1.0))
      (set `self.ObjectRight` null)
      (set `self.SelectedPickup` null))
    (:`else`)))

(fn `PickupLeft`
  (bind _selectedpickup (`self.SelectedPickup`))
  (`/Engine/EditorBlueprintResources/StandardMacros.IsValid` _selectedpickup
    (:`Is Valid`
      (if (not (`/Game/_Game/Blueprints/Components/BPA_Pickup.IsHeld` _selectedpickup))
        (bind _output_get (set `self.ObjectLeft` _selectedpickup))
        (`/Game/_Game/Blueprints/Components/BPA_Pickup.OnPickup` _output_get (`self.HandLeft`) self)
        (set `self.SelectedPickup` null)))))

(fn `PickupRight`
  (bind _selectedpickup (`self.SelectedPickup`))
  (`/Engine/EditorBlueprintResources/StandardMacros.IsValid` _selectedpickup
    (:`Is Valid`
      (if (not (`/Game/_Game/Blueprints/Components/BPA_Pickup.IsHeld` _selectedpickup))
        (bind _output_get (set `self.ObjectRight` _selectedpickup))
        (`/Game/_Game/Blueprints/Components/BPA_Pickup.OnPickup` _output_get (`self.HandRight`) self)
        (set `self.SelectedPickup` null)))))

(fn `SetHands`
  (params (HandRight :type "StaticMeshComponent Object Reference") (HandLeft :type "StaticMeshComponent Object Reference"))
  (set `self.HandRight` HandRight)
  (set `self.HandLeft` HandLeft))